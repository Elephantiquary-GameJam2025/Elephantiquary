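; Animation notify that plays a surface-dependent footstep sound at the animated mesh's location.
; On notify, it traces vertically through the mesh origin against WorldStatic objects and reads the hit's physical surface type.
; Wood, cement, tiles or water each set the global SurfaceType audio parameter (FMOD-style) before the shared Footstep_Sound event plays.
; A missed trace plays nothing.
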(fn `Received_Notify`
  (params (MeshComp :type "SkeletalMeshComponent Object Reference") (Animation :type "AnimSequenceBase Object Reference") (EventReference :type "AnimNotifyEventReference Structure (by ref)"))
  (returns (ReturnValue :type Boolean))
  (locals (LocalMeshComp :type "SkeletalMeshComponent Object Reference"))
  (bind _returnvalue (`SceneComponent.K2_GetComponentLocation` (`local.LocalMeshComp`)))
  (set `local.LocalMeshComp` MeshComp)
  (bind (_outhit _returnvalue_2) (`KismetSystemLibrary.LineTraceSingleForObjects` (+ _returnvalue (0.0 0.0 50.0)) (+ _returnvalue (0.0 0.0 -300.0)) (`|MakeArray` "ObjectTypeQuery1" :!type "EObjectTypeQuery Enum")))
  (if _returnvalue_2
    (switch `EPhysicalSurface` (`GameplayStatics.GetSurfaceType` _outhit)
      (:`SurfaceType1`
        (`FMODBlueprintStatics.SetGlobalParameterByName` "SurfaceType"))
      (:`SurfaceType2`
        (`FMODBlueprintStatics.SetGlobalParameterByName` "SurfaceType" 2.0))
      (:`SurfaceType3`
        (`FMODBlueprintStatics.SetGlobalParameterByName` "SurfaceType" 1.0))
      (:`SurfaceType4`
        (`FMODBlueprintStatics.SetGlobalParameterByName` "SurfaceType" 3.0)))
    (`FMODBlueprintStatics.PlayEventAtLocation` "/Game/Fmod/Events/Character/Footstep/Footstep_Sound.Footstep_Sound" (`KismetMathLibrary.MakeTransform` (`SceneComponent.K2_GetComponentLocation` (`local.LocalMeshComp`)))))
  (return false))