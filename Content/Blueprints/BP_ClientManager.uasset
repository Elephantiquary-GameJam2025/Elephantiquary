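; Client order manager that hands out object requests to BP_ClientSlot actors and validates deliveries.
; Initialize fills every slot with an order from the GameMode, using gameplay tags to give each its room.
; A looping timer polls the Box for released, resting grabbables whose class matches an order.
; Completion frees the slot, notifies the GameMode and starts a random-interval refill timer, which stops when slots are full or on game over.
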(event `CheckOverlappingObjects`
  (bind (_foundobject _linkedclientslot) (`self.CheckForObjectPresence`))
  (`/Engine/EditorBlueprintResources/StandardMacros.IsValid` _foundobject
    (:`Is Valid`
      (`self.OnOrderCompleted` _linkedclientslot _foundobject))))

(event `DebugValidateOrder`
  (`/Game/GameManager/BP_ElephantGameMode.OnAnOrderWasCompleted` (`self.GameMode`) (0.0 0.0 0.0)))

(event `OnOrderCompleted`
  (params (FreedClientSlot :type "/Game/Blueprints/BP_ClientSlot Object Reference") (ObjectDelievered :type "/Game/Blueprints/Objects/BP_GrabbableObject Object Reference"))
  (`/Game/Blueprints/BP_ClientSlot.OrderCompleted` FreedClientSlot)
  (`KismetArrayLibrary.Array_Add` (`self.FreeOrderSlots`) FreedClientSlot)
  (`BlueprintMapLibrary.Map_Add` (`self.OrderSlots`) FreedClientSlot)
  (`|ExecutionSequence`
    (:`then_0`
      (`NiagaraFunctionLibrary.SpawnSystemAtLocation` "/Game/VFX/AchievementSparkles/FX_Achievment_sparkles.FX_Achievment_sparkles" (`SceneComponent.K2_GetComponentLocation` (`/Game/Blueprints/Objects/BP_Object.Mesh` ObjectDelievered)))
      (`/Game/GameManager/BP_ElephantGameMode.OnAnOrderWasCompleted` (`self.GameMode`) (`SceneComponent.K2_GetComponentLocation` (`/Game/Blueprints/Objects/BP_Object.Mesh` ObjectDelievered)))
      (`/Game/Blueprints/Objects/BP_GrabbableObject.OnObjectDelivered` ObjectDelievered))
    (:`then_1`
      (if (not (`KismetSystemLibrary.K2_IsTimerActiveHandle` (`self.NewOrderTimer`)))
        (bind _returnvalue (`KismetSystemLibrary.K2_SetTimerDelegate` (`|CreateDelegate` :!event `OnNewOrderTimerOver`) (`KismetMathLibrary.RandomFloatInRange` (`self.MinOrderInterval`) (`self.MaxOrderInterval`)) true))
        (set `self.NewOrderTimer` _returnvalue)))))

(event `self.ReceiveTick`
  (params (DeltaSeconds :type "Float (single-precision)")))

(event `OnGameOver`
  (`KismetSystemLibrary.K2_ClearAndInvalidateTimerHandle` (`self.NewOrderTimer`)))

(event `OnNewOrderTimerOver`
  (`self.SetUpNewOrder`)
  (if (<= (`KismetArrayLibrary.Array_Length` (`self.FreeOrderSlots`)) 0)
    (`KismetSystemLibrary.K2_ClearAndInvalidateTimerHandle` (`self.NewOrderTimer`))))

(fn `CheckForObjectPresence`
  (returns (FoundObject :type "/Game/Blueprints/Objects/BP_GrabbableObject Object Reference") (LinkedClientSlot :type "/Game/Blueprints/BP_ClientSlot Object Reference"))
  (locals (SlotOrderObject :type "/Game/Blueprints/Objects/BP_GrabbableObject Object Reference") (LinkedOrderSlot :type "/Game/Blueprints/BP_ClientSlot Object Reference"))
  (for _array_element (`PrimitiveComponent.GetOverlappingActors` (`self.Box`) null)
    (bind _asbp_grabbable_object (cast `/Game/Blueprints/Objects/BP_GrabbableObject` _array_element))
    (if (`/Game/Blueprints/Objects/BP_GrabbableObject.IsGrabbed` _asbp_grabbable_object)
      _
      (elif (`/Game/Blueprints/Objects/BP_GrabbableObject.GetIsDelivered` _asbp_grabbable_object)
        _
        (elif (< (`KismetMathLibrary.VSize` (`SceneComponent.GetComponentVelocity` (`/Game/Blueprints/Objects/BP_Object.Mesh` _asbp_grabbable_object))) 1.0)
          (bind _keys (`BlueprintMapLibrary.Map_Keys` (`self.OrderSlots`)))
          (for _array_element_2 _keys
            (set `local.LinkedOrderSlot` _array_element_2)
            (set `local.SlotOrderObject` (`BlueprintMapLibrary.Map_Find` (`self.OrderSlots`) _array_element_2))
            (`/Engine/EditorBlueprintResources/StandardMacros.IsValid` (`local.SlotOrderObject`)
              (:`Is Valid`
                (if (== (`GameplayStatics.GetObjectClass` _asbp_grabbable_object) (`GameplayStatics.GetObjectClass` (`local.SlotOrderObject`)))
                  (return _asbp_grabbable_object (`local.LinkedOrderSlot`))))))))))
  (return null null))

(fn `Initialize`
  (`KismetSystemLibrary.K2_SetTimerDelegate` (`|CreateDelegate` :!event `CheckOverlappingObjects`) 0.25 true)
  (bind _asbp_elephant_game_mode (cast `/Game/GameManager/BP_ElephantGameMode` (`GameplayStatics.GetGameMode`)))
  (bind _output_get (set `self.GameMode` _asbp_elephant_game_mode))
  (add `/Game/GameManager/BP_ElephantGameMode.OnGameOver` _output_get (`|CreateDelegate` :!event `OnGameOver`))
  (bind _outactors (`GameplayStatics.GetAllActorsOfClass` "/Game/Blueprints/BP_ClientSlot.BP_ClientSlot_C"))
  (for _array_element _outactors
    (`BlueprintMapLibrary.Map_Add` (`self.OrderSlots`) _array_element)
    (`KismetArrayLibrary.Array_Add` (`self.FreeOrderSlots`) _array_element)
    (`self.SetUpNewOrder`)))

(fn `SetUpNewOrder`
  (locals (RandomFreeClientSpot :type "/Game/Blueprints/BP_ClientSlot Object Reference"))
  (set `local.RandomFreeClientSpot` (`KismetArrayLibrary.Array_Random` (`self.FreeOrderSlots`)))
  (`KismetArrayLibrary.Array_RemoveItem` (`self.FreeOrderSlots`) (`local.RandomFreeClientSpot`))
  (bind _orderobject (`/Game/GameManager/BP_ElephantGameMode.RequestOrder` (`self.GameMode`)))
  (`BlueprintMapLibrary.Map_Add` (`self.OrderSlots`) (`local.RandomFreeClientSpot`) _orderobject)
  (bind _tags (`/Game/Blueprints/Objects/BP_Object.RetrieveTags` _orderobject))
  (`/Game/Blueprints/BP_ClientSlot.Received Order` (`local.RandomFreeClientSpot`) (`/Game/Blueprints/Objects/BP_GrabbableObject.ObjectPicto` _orderobject) (select `bool` (`BlueprintGameplayTagLibrary.HasTag` _tags (struct :`TagName` "Elephantiquarry.Area.Medieval") true) :`false` (select `bool` (`BlueprintGameplayTagLibrary.HasTag` _tags (struct :`TagName` "Elephantiquarry.Area.Garden") true) :`false` "NewEnumerator2" :`true` "NewEnumerator0" :!type "/Game/Blueprints/GenericEnums/E_RoomTypes Enum") :`true` "NewEnumerator1")))

(fn `UserConstructionScript`)