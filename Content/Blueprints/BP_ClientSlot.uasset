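; BP_ClientSlot is a client slot that announces incoming orders with a ringing phone and shows them on a WBP_ClientOrder widget.
; ReceivedOrder plays the phone ringing animation, waits a fixed delay, then makes the widget appear with the object picto and room style and plays a 2D sound event.
; OrderCompleted hides the widget, whose reference is lazily cast from the OrderWidget component and cached.
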(event `Received Order`
  (params (ObjectPicto :type "Texture Object Reference") (ObjectRoom :type "/Game/Blueprints/GenericEnums/E_RoomTypes Enum" :default "NewEnumerator0"))
  (`SkeletalMeshComponent.PlayAnimation` (`self.SKM_PhoneArma`) "/Game/3Dassets/Anims/Phone/Anim_PhoneRinging.Anim_PhoneRinging" false)
  ;[1 1 1] no control to stop it/know the context after delay. Add a branch/use a timer?
  (`KismetSystemLibrary.Delay` 1.25)
  (bind _orderwidgetref (`self.GetOrderWidgetRef`))
  (`/Game/UI/Widgets/Orders/WBP_ClientOrder.OnAppearing` _orderwidgetref ObjectPicto ObjectRoom)
  (`FMODBlueprintStatics.PlayEvent2D` "/Game/Fmod/Events/Clients/New_Order.New_Order"))

(fn `GetOrderWidgetRef`
  (returns (OrderWidgetRef :type "/Game/UI/Widgets/Orders/WBP_ClientOrder Object Reference"))
  (`/Engine/EditorBlueprintResources/StandardMacros.IsValid` (`self.OrderWidgetRef`)
    (:`Is Valid`
      (return (`self.OrderWidgetRef`)))
    (:`Is Not Valid`
      (bind _aswbp_client_order (cast `/Game/UI/Widgets/Orders/WBP_ClientOrder` (`WidgetComponent.GetWidget` (`self.OrderWidget`))))
      (bind _output_get (set `self.OrderWidgetRef` _aswbp_client_order))
      (return _output_get))))

(fn `OrderCompleted`
  (bind _orderwidgetref (`self.GetOrderWidgetRef`))
  (`/Game/UI/Widgets/Orders/WBP_ClientOrder.OnDisappearing` _orderwidgetref))

(fn `UserConstructionScript`)