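; BP_ClientSpot is a client's drop-off point that shows an order and detects its delivery.
; Initialize stores the order object, then after a delay plays a sound and fills the order widget's picture and tag-based bubble style.
; A looping timer polls box overlaps for the order's class; if the stored object isn't grabbed, it spawns sparkles, destroys that object, fires order completion and increments the count.
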(event `self.ReceiveBeginPlay`
  (`KismetSystemLibrary.K2_SetTimerDelegate` (delegate `CheckOverlappingObjects`) 1.0 true))

(event `CheckOverlappingObjects`
  (bind _returnvalue (`SceneComponent.K2_GetComponentLocation` (`/Game/Blueprints/Objects/BP_Object.Mesh` (`self.CurrentOrderObject`))))
  (for _array_element (`PrimitiveComponent.GetOverlappingActors` (`self.Box`) null)
    (`/Engine/EditorBlueprintResources/StandardMacros.IsValid` (`self.CurrentOrderObject`)
      (:`Is Valid`
        (if (== (`GameplayStatics.GetObjectClass` _array_element) (`GameplayStatics.GetObjectClass` (`self.CurrentOrderObject`)))
          (if (not (`/Game/Blueprints/Objects/BP_GrabbableObject.isGrabbed` (`self.CurrentOrderObject`)))
            (`NiagaraFunctionLibrary.SpawnSystemAtLocation` "/Game/VFX/AchievementSparkles/FX_Achievment_sparkles.FX_Achievment_sparkles" _returnvalue)
            (set `self.OrderCapturedLocation` _returnvalue)
            (`self.K2_DestroyActor` (`self.CurrentOrderObject`))
            (set `self.CurrentOrderObject` null)
            (`self.OnOrderComplete` self)
            (`self.IncreaseOrderCount`)))))))

(event `InitializeNewOrder`
  (bind _currentorderobject (`self.CurrentOrderObject`))
  (`KismetSystemLibrary.Delay` 1.0)
  (`FMODBlueprintStatics.PlayEvent2D` "/Game/Fmod/Events/Clients/New_Order.New_Order")
  (bind _orderwidgetref (`self.GetOrderWidgetRef`))
  (`/Game/UI/Widgets/Orders/WBP_ClientOrder.SetOrderImage` _orderwidgetref (`/Game/Blueprints/Objects/BP_GrabbableObject.ObjectPicto` _currentorderobject))
  (`self.DebugTextPrint` _currentorderobject _currentorderobject _orderwidgetref)
  (bind _aswbp_client_order (cast `/Game/UI/Widgets/Orders/WBP_ClientOrder` (`WidgetComponent.GetWidget` (`self.OrderWidget`))))
  (bind _tags (`/Game/Blueprints/Objects/BP_Object.RetrieveTags` (`self.CurrentOrderObject`)))
  ;[1 1 1] Clearly improvable, feel free to do so
  (`/Game/UI/Widgets/Orders/WBP_ClientOrder.SetSpeechBubbleStyle` _aswbp_client_order (select `bool` (`BlueprintGameplayTagLibrary.HasTag` _tags (struct :`TagName` "Elephantiquarry.Area.Antiquities") true) :`false` (select `bool` (`BlueprintGameplayTagLibrary.HasTag` _tags (struct :`TagName` "Elephantiquarry.Area.Greenhouse") true) :`false` "NewEnumerator2" :`true` "NewEnumerator0" :!type "/Game/Blueprints/GenericEnums/E_RoomTypes Enum") :`true` "NewEnumerator1")))

(fn `DebugTextPrint`
  (params (Object :type "Object Object Reference") (self2 :type "/Game/Blueprints/Objects/BP_GrabbableObject Object Reference") (self3 :type "/Game/UI/Widgets/Orders/WBP_ClientOrder Object Reference"))
  (bind _debugtext (`/Game/UI/Widgets/Orders/WBP_ClientOrder.DebugText` self3))
  (if (== (`/Game/Blueprints/Objects/BP_GrabbableObject.ObjectPicto` self2) "/Game/UI/UI_Ressource/Textures/OldPropsIcon/lil_crow.lil_crow")
    (set `TextBlock.Text` (`KismetTextLibrary.Conv_StringToText` (`KismetSystemLibrary.GetDisplayName` Object)) _debugtext)
    (`Widget.SetVisibility` _debugtext "Visible")
    (else
      (`Widget.SetVisibility` _debugtext "Collapsed"))))

(fn `GetOrderWidgetRef`
  (returns (OrderWidgetRef :type "/Game/UI/Widgets/Orders/WBP_ClientOrder Object Reference"))
  (`/Engine/EditorBlueprintResources/StandardMacros.IsValid` (`self.OrderWidgetRef`)
    (:`Is Valid`
      (return (`self.OrderWidgetRef`)))
    (:`Is Not Valid`
      (bind _aswbp_client_order (cast `/Game/UI/Widgets/Orders/WBP_ClientOrder` (`WidgetComponent.GetWidget` (`self.OrderWidget`))))
      (bind _output_get (set `self.OrderWidgetRef` _aswbp_client_order))
      (return _output_get))))

(fn `IncreaseOrderCount`
  (set `self.OrderCount` (+ (`self.OrderCount`) 1)))

(fn `Initialize`
  (params (OrderObject :type "/Game/Blueprints/Objects/BP_GrabbableObject Object Reference") (OrderData :type "/Game/DataTables/ClientOrders/S_ClientOrderDataRow Structure"))
  ;[1 1 1] we keep order data cause we might need it later
  (set `self.CurrentOrderObject` OrderObject)
  (`self.InitializeNewOrder`))

(fn `UserConstructionScript`)