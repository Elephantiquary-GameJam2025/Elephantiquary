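; BP_ModularStructure is a level-design actor that builds a modular structure whose pieces can each use a Neutral, Pirate, Medieval or Garden style.
; The construction script gathers the static mesh children of MeshParent and resizes the StructureTypes array to match their count.
; Each component then gets the mesh that GetStructureMeshByStyle selects for the style at its index.
; All work happens at construction, with no active runtime event logic.
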(fn `GetStructureMeshByStyle`
  (params (Style :type "/Game/Blueprints/LD/E_StructureStyles Enum" :default "NewEnumerator3"))
  (returns (Mesh :type "StaticMesh Object Reference"))
  (return (select `/Game/Blueprints/LD/E_StructureStyles` Style :`NewEnumerator3` (`self.NeutralMesh`) :`NewEnumerator0` (`self.PirateMesh`) :`NewEnumerator1` (`self.MedievalMesh`) :`NewEnumerator2` (`self.GardenMesh`))))

(fn `UserConstructionScript`
  (`KismetArrayLibrary.Array_Clear` (`self.StructureMeshes`))
  (for _array_element (`SceneComponent.GetChildrenComponents` (`self.MeshParent`) false)
    (bind _asstatic_mesh_component (cast `StaticMeshComponent` _array_element))
    (`KismetArrayLibrary.Array_Add` (`self.StructureMeshes`) _asstatic_mesh_component))
  (`KismetArrayLibrary.Array_Resize` (`self.StructureTypes`) (`KismetArrayLibrary.Array_Length` (`self.StructureMeshes`)))
  (for (_array_element_2 _array_index) (`self.StructureMeshes`)
    (`StaticMeshComponent.SetStaticMesh` _array_element_2 (`self.GetStructureMeshByStyle` (`|GetArrayItem` (`self.StructureTypes`) _array_index)))))