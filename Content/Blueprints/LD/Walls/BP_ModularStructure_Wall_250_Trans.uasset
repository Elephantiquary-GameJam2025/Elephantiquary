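; Modular 250-unit transition wall piece for level design, offering Exterior, Medieval, Music and Pirate visual styles.
; It keeps a per-index array of wall styles and maps each entry to the matching style mesh.
; A helper resizes the style array; the event graph holds only disabled stubs and the construction script just calls the parent.
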(fn `GetMeshByIndex`
  (params (Index :type Integer))
  (returns (Mesh :type "StaticMesh Object Reference"))
  (return (select `/Game/Blueprints/LD/E_WallsStyles` (`|GetArrayItem` (`self.WallsStyles`) Index) :`NewEnumerator0` (`self.ExteriorMesh`) :`NewEnumerator1` (`self.MedievalMesh`) :`NewEnumerator2` (`self.MusicMesh`) :`NewEnumerator3` (`self.PirateMesh`))))

(fn `ResizeEnumArray`
  (params (NewArraySize :type Integer))
  (`KismetArrayLibrary.Array_Resize` (`self.WallsStyles`) NewArraySize))

(fn `UserConstructionScript`
  (`parent.UserConstructionScript`))