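; Modular level-design Blueprint that lets each of its mesh pieces switch between Exterior, Medieval, Garden, Pirate and Hub visual styles.
; The Construction Script gathers the static mesh children of ModularMeshesParent and resizes the StructureStyles array to match, giving one style entry per piece.
; Each piece then receives the mesh for its chosen style, or that style's variation when flagged.
; No runtime logic exists.
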(fn `UserConstructionScript`
  (`KismetArrayLibrary.Array_Clear` (`self.StructureMeshes`))
  (for _array_element (`SceneComponent.GetChildrenComponents` (`self.ModularMeshesParent`) false)
    (bind _asstatic_mesh_component (cast `StaticMeshComponent` _array_element))
    (`KismetArrayLibrary.Array_Add` (`self.StructureMeshes`) _asstatic_mesh_component))
  (`KismetArrayLibrary.Array_Resize` (`self.StructureStyles`) (`KismetArrayLibrary.Array_Length` (`self.StructureMeshes`)))
  (for (_array_element_2 _array_index) (`self.StructureMeshes`)
    (bind (_output_structurestyle _output_isusingmeshvariation) (break `/Game/Blueprints/LD_Blueprints/S_StructureData` (`|GetArrayItem` (`self.StructureStyles`) _array_index)))
    (`StaticMeshComponent.SetStaticMesh` _array_element_2 (select `/Game/Blueprints/LD_Blueprints/E_StructureStyles` _output_structurestyle :`NewEnumerator0` (select `bool` _output_isusingmeshvariation :`false` (`self.ExteriorMesh`) :`true` (`self.ExteriorMeshVariation`)) :`NewEnumerator1` (select `bool` _output_isusingmeshvariation :`false` (`self.MedievalMesh`) :`true` (`self.MedievalMeshVariation`)) :`NewEnumerator2` (select `bool` _output_isusingmeshvariation :`false` (`self.GardenMesh`) :`true` (`self.GardenMeshVariation`)) :`NewEnumerator3` (select `bool` _output_isusingmeshvariation :`false` (`self.PirateMesh`) :`true` (`self.PirateMeshVariation`)) :`NewEnumerator4` (select `bool` _output_isusingmeshvariation :`false` (`self.HubMesh`) :`true` (`self.HubMeshVariation`))))))