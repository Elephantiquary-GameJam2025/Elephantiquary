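; Abstract base Blueprint for modular level-design structures, meant to be subclassed rather than placed in the world.
; The construction script gathers static mesh children of ModularMeshesParent into StructureMeshes, asks ResizeEnumArray to match that count, then assigns each mesh through GetMeshByIndex.
; Children override those two functions; the base versions only print a red on-screen error flagging a missing override or direct placement.
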(fn `GetMeshByIndex`
  (params (Index :type Integer))
  (returns (Mesh :type "StaticMesh Object Reference"))
  (`self.PrintNotOveriddenError`)
  (return null))

(fn `PrintNotOveriddenError`
  (`KismetSystemLibrary.PrintString` "Error: Child of ModularStructure is not overiding all the functions it should or ModularStructure has been drag and dropped into the world (it shouldn't)" true true (struct :`R` 1.0 :`A` 1.0) 12.0))

(fn `ResizeEnumArray`
  (params (NewArraySize :type Integer))
  (`self.PrintNotOveriddenError`))

(fn `UserConstructionScript`
  (`KismetArrayLibrary.Array_Clear` (`self.StructureMeshes`))
  (for _array_element (`SceneComponent.GetChildrenComponents` (`self.ModularMeshesParent`) false)
    (bind _asstatic_mesh_component (cast `StaticMeshComponent` _array_element))
    (`KismetArrayLibrary.Array_Add` (`self.StructureMeshes`) _asstatic_mesh_component))
  (`self.ResizeEnumArray` (`KismetArrayLibrary.Array_Length` (`self.StructureMeshes`)))
  (for (_array_element_2 _array_index) (`self.StructureMeshes`)
    (`StaticMeshComponent.SetStaticMesh` _array_element_2 (`self.GetMeshByIndex` _array_index))))