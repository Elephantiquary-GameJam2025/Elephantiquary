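; BP_BreakableObject is a physics prop that shatters on hard impacts and costs the player level time when it breaks.
; After a short spawn invulnerability timer, mesh hits whose impulse exceeds a threshold scaled by mass and a toughness multiplier trigger the break.
; Breaking, if allowed, spawns a Niagara effect, plays an FMOD sound, reduces BP_TopDownGameMode's level duration, then fires OnObjectDestroyed and destroys the actor.
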(event `self.ReceiveBeginPlay`
  (`parent.ReceiveBeginPlay`)
  (`KismetSystemLibrary.K2_SetTimerDelegate` (delegate `StopInvulnerability`) 3.0))

(event `StopInvulnerability`
  (set `self.IsVulnerable` true))

(event `self.Mesh.OnComponentHit`
  (params (HitComponent :type "PrimitiveComponent Object Reference") (OtherActor :type "Actor Object Reference") (OtherComp :type "PrimitiveComponent Object Reference") (NormalImpulse :type "Vector Structure") (Hit :type "HitResult Structure (by ref)"))
  (if (`self.IsVulnerable`)
    (if (> (`KismetMathLibrary.VSize` NormalImpulse) (* (`PrimitiveComponent.GetMass` (`self.Mesh`)) 70.0 (`self.ToughnessMultiplier`)))
      (`self.BreakObject`))))

(event `BreakObject`
  (if (`self.IsAllowedToBreak`)
    (`NiagaraFunctionLibrary.SpawnSystemAtLocation` "/Game/VFX/PropsOrdering/FX_Props_Ordering_Diseapper.FX_Props_Ordering_Diseapper" (`SceneComponent.K2_GetComponentLocation` (`self.Mesh`)))
    (`FMODAudioComponent.Play` (`self.FMODBreak`))
    (`|ExecutionSequence`
      (:`then_0`
        (bind _asbp_top_down_game_mode (cast `/Game/GameManager/BP_TopDownGameMode` (`GameplayStatics.GetGameMode`)))
        (`/Game/GameManager/BP_TopDownGameMode.DecreaseLevelDuration` _asbp_top_down_game_mode (`self.TimeLostOnBreak`) (`SceneComponent.K2_GetComponentLocation` (`self.Mesh`))))
      (:`then_1`
        (`self.OnObjectDestroyed`)
        (`self.K2_DestroyActor`)))))

(fn `UserConstructionScript`
  (`parent.UserConstructionScript`))