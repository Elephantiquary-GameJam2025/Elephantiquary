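; Physics object the player can target, grab and deliver, with the Grabable collision profile applied by gameplay tag.
; Targeting and grabbing swap outline overlay materials, and grabbing also changes linear damping.
; Velocity drives FMOD friction and impact sounds, enabled after a startup delay, with a cooldown on impacts.
; Delivery freezes physics, spawns a cardboard box and floor-traced pivot, then shrinks the object around that pivot via timeline and destroys all three.
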(event `self.ReceiveBeginPlay`
  (`parent.ReceiveBeginPlay`)
  (`|ExecutionSequence`
    (:`then_0`
      (if (`BlueprintGameplayTagLibrary.HasTag` (`self.GameplayTagContainer`) (struct :`TagName` "Elephantiquarry.Object.ObjectType.Grabable"))
        (`PrimitiveComponent.SetCollisionProfileName` (`self.Mesh`) "Grabable" true)))
    (:`then_1`
      (bind _asbp_elephant_game_mode (cast `/Game/GameManager/BP_ElephantGameMode` (`GameplayStatics.GetGameMode`)))
      (add `/Game/GameManager/BP_ElephantGameMode.OnGameOver` _asbp_elephant_game_mode (`|CreateDelegate` :!event `OnGameOver`))
      (`KismetSystemLibrary.K2_SetTimerDelegate` (delegate `OnPhysicsSoundActivated`) (`self.PhysicsSoundActivationPeriod`)))))

(event `OnPhysicsSoundActivated`
  (set `self.CanPhysicsSoundsBePlayed` true))

(event `SetAsTarget`
  (params (Result :type Boolean))
  (if (`self.IsGrabbed`)
    _
    (elif Result
      (`MeshComponent.SetOverlayMaterial` (`self.Mesh`) "/Game/3Dassets/Materials/MI_OutlineSelected.MI_OutlineSelected")
      (else
        (`MeshComponent.SetOverlayMaterial` (`self.Mesh`) null)))))

(event `self.ReceiveTick`
  (params (DeltaSeconds :type "Float (single-precision)"))
  (`parent.ReceiveTick` DeltaSeconds)
  ;[1 1 1] Update Volume And intensity or stop Friction
  (if (> (`self.GetObjectVelocityLength`) 0.0)
    (`FMODAudioComponent.SetParameter` (`self.FMODImpact`) "Volume" (`KismetMathLibrary.FClamp` (`self.GetObjectVelocityLength`) 0.0 1500.0))
    (`FMODAudioComponent.SetParameter` (`self.FMODFriction`) "Volume" (`KismetMathLibrary.FClamp` (`self.GetObjectVelocityLength`) 0.0 1500.0))
    (`FMODAudioComponent.SetParameter` (`self.FMODFriction`) "Velocity" (`KismetMathLibrary.FClamp` (`self.GetObjectVelocityLength`) 0.0 1500.0))
    (else
      (bind _returnvalue (`FMODAudioComponent.IsPlaying` (`self.FMODFriction`)))
      (if _returnvalue
        (`FMODAudioComponent.Stop` (`self.FMODFriction`))
        (goto _label :!via `Reset`)))))

(event `self.Mesh.OnComponentHit`
  (params (HitComponent :type "PrimitiveComponent Object Reference") (OtherActor :type "Actor Object Reference") (OtherComp :type "PrimitiveComponent Object Reference") (NormalImpulse :type "Vector Structure") (Hit :type "HitResult Structure (by ref)"))
  (bind _returnvalue (`KismetMathLibrary.FClamp` (`KismetMathLibrary.VSize` (`SceneComponent.GetComponentVelocity` (`self.Mesh`))) 0.0 1500.0))
  ;[1 1 1] Impact & Friction Audio on hit
  (if (`self.CanPhysicsSoundsBePlayed`)
    (`|ExecutionSequence`
      (:`then_0`
        (`/Engine/EditorBlueprintResources/StandardMacros.DoOnce` false :!label _label
          (:`Completed`
            (`FMODAudioComponent.Play` (`self.FMODFriction`)))))
      (:`then_1`
        (if (>= _returnvalue (`self.VelocityForImpactSound`))
          (`/Engine/EditorBlueprintResources/StandardMacros.DoOnce` false :!label _label_2
            (:`Completed`
              (`FMODAudioComponent.SetParameter` (`self.FMODImpact`) "Volume" _returnvalue)
              (`FMODAudioComponent.Play` (`self.FMODImpact`))
              (`KismetSystemLibrary.Delay` 0.3)
              (goto _label_2 :!via `Reset`))))))))

(event `OnGameOver`
  (`FMODAudioComponent.Stop` (`self.FMODFriction`)))

(event `OnObjectDelivered`
  (bind _returnvalue (`KismetMathLibrary.FMax` (`CurveFloat.GetFloatValue` (`self.ScaleDownCurve`) (`TimelineComponent.GetPlaybackPosition` (`self.ObjectDeliveredTimeline`))) 0.01))
  (set `self.IsDelivered` true)
  (`PrimitiveComponent.SetSimulatePhysics` (`self.Mesh`) false)
  (`TimelineComponent.SetPlayRate` (`self.ObjectDeliveredTimeline`) (/ 1.0 (`self.ObjectDeliveryDuration`)))
  (bind _lowestcenterpoint (`self.GetsLowestCenterPoint`))
  (bind _returnvalue_2 (`|SpawnActorFromClass` "/Game/Blueprints/Objects/BP_DeliveryObjectAnchor.BP_DeliveryObjectAnchor_C" (`KismetMathLibrary.MakeTransform` _lowestcenterpoint) "AlwaysSpawn" "MultiplyWithRoot" null null))
  (set `self.DeliveredScalePivotPoint` _returnvalue_2)
  (`self.K2_AttachToActor` (`self.DeliveredScalePivotPoint`) "None" "KeepWorld" "KeepRelative" "KeepRelative")
  (bind _lowestcenterpoint_2 (`self.GetsLowestCenterPoint`))
  (bind _returnvalue_3 (`|SpawnActorFromClass` "/Game/Blueprints/Objects/BP_CardboardBox.BP_CardboardBox_C" (`KismetMathLibrary.MakeTransform` _lowestcenterpoint_2 (`KismetMathLibrary.MakeRotFromZX` (`KismetMathLibrary.Vector_Up`) (`self.GetActorForwardVector`))) "AlwaysSpawn" "MultiplyWithRoot" null null))
  (`Timeline|ObjectDeliveredTimeline` :!via `PlayFromStart`
    (:`Update`
      (`self.SetActorScale3D` (`self.DeliveredScalePivotPoint`) (`KismetMathLibrary.MakeVector` _returnvalue _returnvalue _returnvalue)))
    (:`Finished`
      (`self.K2_DestroyActor` _returnvalue_3)
      (`self.K2_DestroyActor` (`self.DeliveredScalePivotPoint`))
      (`self.K2_DestroyActor`))))

(fn `GetIsDelivered`
  (returns (IsDelivered :type Boolean))
  (return (`self.IsDelivered`)))

(fn `GetObjectVelocityLength`
  (returns (ReturnValue :type "Float (double-precision)"))
  (return (`KismetMathLibrary.VSize` (`SceneComponent.GetComponentVelocity` (`self.Mesh`)))))

(fn `GetsLowestCenterPoint`
  (returns (LowestCenterPoint :type "Vector Structure"))
  (bind _origin (`KismetSystemLibrary.GetComponentBounds` (`self.Mesh`)))
  (bind _outhit (`KismetSystemLibrary.LineTraceSingleForObjects` :`Start` _origin :`End` (- _origin (0.0 0.0 1000.0)) :`ObjectTypes` (`|MakeArray` "ObjectTypeQuery1" :!type "EObjectTypeQuery Enum") :`DrawTime` 15.0))
  (return (`.Location` (`GameplayStatics.BreakHitResult` _outhit))))

(fn `SetGrabbed`
  (params (isGrabbed :type Boolean))
  (if isGrabbed
    (set `self.IsGrabbed` true)
    (`PrimitiveComponent.SetLinearDamping` (`self.Mesh`) (/ (`PrimitiveComponent.GetLinearDamping` (`self.Mesh`)) (`self.LinearDampingMultiplier`)))
    (`MeshComponent.SetOverlayMaterial` (`self.Mesh`) "/Game/3Dassets/Materials/MI_OutlineGrabbed.MI_OutlineGrabbed")
    (else
      (set `self.IsGrabbed` false)
      (`PrimitiveComponent.SetLinearDamping` (`self.Mesh`) (* (`PrimitiveComponent.GetLinearDamping` (`self.Mesh`)) (`self.LinearDampingMultiplier`)))
      (`MeshComponent.SetOverlayMaterial` (`self.Mesh`) null))))

(fn `UserConstructionScript`
  (`parent.UserConstructionScript`))