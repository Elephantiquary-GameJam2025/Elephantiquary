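; BP_Object is a gameplay-tagged world object with a physics mesh that can return to its starting transform.
; BeginPlay caches the mesh's world transform and disables decals on it; ReturnToBaseTransform teleports it back and clears its velocities.
; Tags can be appended and retrieved, and the construction script shows a billboard for objects tagged HardToReach.
; GetPhysicsObject exposes the mesh, while UpdateDecalOrientation is empty.
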(event `self.ReceiveBeginPlay`
  (bind _mesh (`self.Mesh`))
  (set `self.MeshInitialTransform` (`SceneComponent.K2_GetComponentToWorld` _mesh))
  (`PrimitiveComponent.SetReceivesDecals` _mesh false))

(event `/Game/Player/I_GameplayTagContainer.AddTags`
  (params (Tags :type "GameplayTagContainer Structure"))
  (`BlueprintGameplayTagLibrary.AppendGameplayTagContainers` (`self.GameplayTagContainer`) Tags))

(event `UpdateDecalOrientation`)

(fn `GetPhysicsObject`
  (returns (Object :type "StaticMeshComponent Object Reference"))
  (return (`self.Mesh`)))

(fn `RetrieveTags`
  (returns (Tags :type "GameplayTagContainer Structure"))
  (return (`self.GameplayTagContainer`)))

(fn `ReturnToBaseTransform`
  (`SceneComponent.K2_SetWorldTransform` (`self.Mesh`) (`self.MeshInitialTransform`) false true)
  (`PrimitiveComponent.SetAllPhysicsLinearVelocity` (`self.Mesh`) (0.0 0.0 0.0) false)
  (`PrimitiveComponent.SetAllPhysicsAngularVelocityInDegrees` (`self.Mesh`) (0.0 0.0 0.0) false))

(fn `UserConstructionScript`
  (`SceneComponent.SetVisibility` (`self.HardToReachBillboard`) (`BlueprintGameplayTagLibrary.HasTag` (`self.GameplayTagContainer`) (struct :`TagName` "Elephantiquarry.Special.HardToReach") true) false))