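; BP_VaseMing is a breakable Ming vase object that extends a parent breakable-object Blueprint.
; On BreakObject it plays an FMOD break sound and spawns BP_BrokenMingVase at the mesh's transform.
; It aligns the spawned breakable component to that transform, applies an upward impulse to scatter it, then calls the parent break logic.
; An FX asset setter is left unconnected and never runs.
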(event `self.BreakObject`
  (bind _returnvalue (`SceneComponent.K2_GetComponentToWorld` (`self.Mesh`)))
  (`FMODAudioComponent.Play` (`self.FMODBreak`))
  (bind _returnvalue_2 (`|SpawnActorFromClass` "/Game/Blueprints/Objects/BP_BrokenMingVase.BP_BrokenMingVase_C" _returnvalue "Undefined" "MultiplyWithRoot" null null))
  (bind _gc_bp_vasemingbreakable (`/Game/Blueprints/Objects/BP_BrokenMingVase.GC_BP_VaseMingBreakable` _returnvalue_2))
  (`SceneComponent.K2_SetWorldTransform` _gc_bp_vasemingbreakable _returnvalue false false)
  (`PrimitiveComponent.AddImpulse` _gc_bp_vasemingbreakable (0.0 0.0 2000.0) "None" false)
  (`parent.BreakObject`))

(fn `UserConstructionScript`
  (`parent.UserConstructionScript`))