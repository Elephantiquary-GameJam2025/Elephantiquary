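; SD_ImpactTest is a physics sound test actor that drives FMOD friction and impact audio from its mesh's speed.
; Tick feeds clamped speed into both sounds' Volume and friction's Velocity, stopping friction when the mesh is still.
; Hits start friction through a DoOnce that re-arms when Tick stops it.
; Fast hits also play the impact sound, gated by a second DoOnce with a short delayed reset as cooldown.
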(event `self.ReceiveTick`
  (params (DeltaSeconds :type "Float (single-precision)"))
  (bind _fmodfriction_0 (`self.FMODFriction_0`))
  (bind _fmodfriction_0_2 (`self.FMODFriction_0`))
  (bind _returnvalue (`KismetMathLibrary.VSize` (`SceneComponent.GetComponentVelocity` (`self.Mesh`))))
  (bind _returnvalue_2 (`KismetMathLibrary.FClamp` _returnvalue 0.0 1500.0))
  (if (> _returnvalue 0.0)
    (`FMODAudioComponent.SetParameter` _fmodfriction_0_2 "Volume" _returnvalue_2)
    (`FMODAudioComponent.SetParameter` (`self.FMODImpact_0`) "Volume" _returnvalue_2)
    (`FMODAudioComponent.SetParameter` _fmodfriction_0_2 "Velocity" _returnvalue_2)
    (else
      (bind _returnvalue_3 (`FMODAudioComponent.IsPlaying` _fmodfriction_0))
      (if _returnvalue_3
        (`FMODAudioComponent.Stop` _fmodfriction_0)
        (goto _label :!via `Reset`)))))

(event `self.Mesh.OnComponentHit`
  (params (HitComponent :type "PrimitiveComponent Object Reference") (OtherActor :type "Actor Object Reference") (OtherComp :type "PrimitiveComponent Object Reference") (NormalImpulse :type "Vector Structure") (Hit :type "HitResult Structure (by ref)"))
  (bind _returnvalue (`KismetMathLibrary.FClamp` (`KismetMathLibrary.VSize` (`SceneComponent.GetComponentVelocity` (`self.Mesh`))) 0.0 1500.0))
  (`|ExecutionSequence`
    (:`then_0`
      (`/Engine/EditorBlueprintResources/StandardMacros.DoOnce` false :!label _label
        (:`Completed`
          (`FMODAudioComponent.Play` (`self.FMODFriction_0`)))))
    (:`then_1`
      (if (>= _returnvalue 1000.0)
        (`/Engine/EditorBlueprintResources/StandardMacros.DoOnce` false :!label _label_2
          (:`Completed`
            (`FMODAudioComponent.SetParameter` (`self.FMODImpact_0`) "Volume" _returnvalue)
            (`FMODAudioComponent.Play` (`self.FMODImpact_0`))
            (`KismetSystemLibrary.Delay` 0.3)
            (goto _label_2 :!via `Reset`)))))))

(fn `UserConstructionScript`)