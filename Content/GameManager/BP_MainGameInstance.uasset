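; BP_MainGameInstance is a Game Instance that holds the current level index and the per-level result data for the game.
; GetLevelData returns the cached results, or loads them from the save through GetSave when the cache is empty, and reports whether a save existed.
; SetLevelData passes a result to OverrideLevelSavedDataIfBetter, then returns whether it beat the previous one along with that level's saved entry.
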(event `/Game/GameManager/I_ElephantInstance.SetCurrentLevelIndex`
  (params (Index :type Integer))
  (set `self.CurrentLevelIndex` Index))

(fn `GetCurrentLevelIndex`
  (returns (LevelIndex :type Integer))
  (return (`self.CurrentLevelIndex`)))

(fn `GetLevelData`
  (returns (DidSaveFileExist :type Boolean) (LevelData :type "Map of Integer to /Game/DataTables/LevelResult/S_LevelResult Structure"))
  (if (> (`BlueprintMapLibrary.Map_Length` (`self.LevelData`)) 0)
    (return true (`self.LevelData`))
    (else
      (bind (_didsavefileexist _levelresults) (`/Game/GameManager/BPFL_SaveHandler.GetSave`))
      (set `self.LevelData` _levelresults)
      (return _didsavefileexist _levelresults))))

(fn `SetLevelData`
  (params (LevelIndex :type Integer) (LevelData :type "/Game/DataTables/LevelResult/S_LevelResult Structure"))
  (returns (ResultWasBetterThanBefore :type Boolean) (UpdatedLevelData :type "/Game/DataTables/LevelResult/S_LevelResult Structure"))
  (bind (_resultwasbetter _datasaved) (`/Game/GameManager/BPFL_SaveHandler.OverrideLevelSavedDataIfBetter` LevelIndex LevelData))
  (return _resultwasbetter (`BlueprintMapLibrary.Map_Find` _datasaved LevelIndex)))