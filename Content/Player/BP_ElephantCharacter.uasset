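; Physics-driven player elephant that moves by forces, turns by torque and grabs objects with its trunk.
; An overlap component gathers grabbable candidates; Tick highlights the best by facing angle, then distance, after sphere and line trace occlusion checks.
; Grabbing lerps the object to the trunk via a PhysicsHandle and timeline while turning the capsule toward it.
; Object mass scales reach time, speed, rotation and carry height; look input steers while carrying.
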(event `self.ReceiveBeginPlay`
  ;[1 0.1451 0.8144] Updates & Collisions
  (`TimelineComponent.SetPlayRate` (`self.ReachTrunkTimeline`) 5.0)
  (`self.ResetRotationAndSpeed`)
  (`KismetSystemLibrary.Delay` 0.2)
  (`SceneComponent.SetHiddenInGame` (`self.Mesh`) false false)
  (`ActorComponent.K2_DestroyComponent` (`self.Plane`)))

(event `/Game/Player/I_InteractibleCharacter.Move`
  (params (Value :type "Vector2D Structure"))
  (bind (_movex _movey) (`self.ProcessAndDampenMoveInput` Value))
  ;[0.2131 0.9103 1] Actions
  ;;[1 1 1] Move Behavior
  (if (`self.GrabbingTransition`)
    _
    (elif (> (`KismetMathLibrary.VSize2DSquared` Value) 0.0)
      (`/Engine/EditorBlueprintResources/StandardMacros.IsValid` (`self.GetController`)
        (:`Is Valid`
          (`|ExecutionSequence`
            (:`then_0`
              (set `self.LastInput` (`KismetMathLibrary.MakeVector2D` _movex _movey)))
            (:`then_1`
              (`PrimitiveComponent.AddForce` (`self.CapsuleCollision`) (`self.ScaleMoveInputToForce` _movex _movey) "None" false))
            (:`then_2`
              ;;;[1 1 1] If no input is pressed, we ignore the velocity based rotation
              (if (> (`KismetMathLibrary.VSize2DSquared` (`self.LastInput`)) 0.0)
                ;;;[1 1 1] Velocity based rotation of the character
                (if (and (`self.RotatesAutomatically`) (not (`self.isGrabbing`)))
                  (`PrimitiveComponent.AddTorqueInDegrees` (`self.CapsuleCollision`) (`KismetMathLibrary.MakeVector` 0.0 0.0 (`self.ProcessVelocityToTorqueValue`)) "None" true)))))))
      (else
        (set `self.LastInput` (0.0 0.0))))))

(event `self.ReceiveTick`
  (params (DeltaSeconds :type "Float (single-precision)"))
  (bind _grabbabletarget (`self.GrabbableTarget`))
  ;[1 0.1451 0.8144] Updates & Collisions
  ;;[1 1 1] If we're currently not grabbing, we are constantly searching for the object to highlight as grabbable
  (if (`self.isGrabbing`)
    ;;[1 1 1] If we are grabbing, we stop looking for objects and instead update the location the grabbed object should be, unless we are in grabbing transition (meaning we grabbed it but it didn't yet reach its grabbed position)
    (if (not (`self.GrabbingTransition`))
      (`PhysicsHandleComponent.SetTargetLocation` (`self.PhysicsHandle`) (`KismetMathLibrary.TransformLocation` (`SceneComponent.K2_GetComponentToWorld` (`self.CapsuleCollision`)) (`self.RagdollTargetLoc`)))
      (`self.UpdateTrunkPosition` (`SceneComponent.K2_GetComponentLocation` (`self.GrabbingPlace`))))
    (`/Engine/EditorBlueprintResources/StandardMacros.IsValid` (`self.GrabbableTarget`) :!label _label
      (:`Is Valid`
        (`/Game/Blueprints/Objects/BP_GrabbableObject.SetAsTarget` (`self.GrabbableTarget`) false)
        (set `self.GrabbableTarget` null)))
    (else
      (bind _object (`self.GetIdealGrabbableObject`))
      (`/Engine/EditorBlueprintResources/StandardMacros.IsValid` _object
        (:`Is Valid`
          (`/Engine/EditorBlueprintResources/StandardMacros.IsValid` _grabbabletarget
            (:`Is Valid`
              (`/Game/Blueprints/Objects/BP_GrabbableObject.SetAsTarget` _grabbabletarget false)
              (`/Game/Blueprints/Objects/BP_GrabbableObject.SetAsTarget` _object false))
            (:`Is Not Valid`
              _))
          (bind _output_get (set `self.GrabbableTarget` _object))
          (`/Game/Blueprints/Objects/BP_GrabbableObject.SetAsTarget` _output_get true))
        (:`Is Not Valid`
          (goto _label))))))

(event `self.Interactible.OnComponentBeginOverlap`
  (params (OverlappedComponent :type "PrimitiveComponent Object Reference") (OtherActor :type "Actor Object Reference") (OtherComp :type "PrimitiveComponent Object Reference") (OtherBodyIndex :type Integer) (bFromSweep :type Boolean) (SweepResult :type "HitResult Structure (by ref)"))
  ;[1 0.1451 0.8144] Updates & Collisions
  ;;[1 1 1] If an object enters our Interactible Capsule, this means it is a candidate to be grabbable, so we check if it has the right conditions and add it to the grabbable candidates
  (if (`KismetSystemLibrary.DoesImplementInterface` OtherActor "/Game/Player/I_GameplayTagContainer.I_GameplayTagContainer_C")
    (bind _tags (message `/Game/Player/I_GameplayTagContainer.RetrieveTags` OtherActor))
    (if (`BlueprintGameplayTagLibrary.HasTag` _tags (struct :`TagName` "Elephantiquarry.Object.ObjectType.Grabable") true)
      (bind _asbp_grabbable_object (cast `/Game/Blueprints/Objects/BP_GrabbableObject` OtherActor))
      (if (`/Game/Blueprints/Objects/BP_GrabbableObject.IsGrabbable` _asbp_grabbable_object)
        (`KismetArrayLibrary.Array_Add` (`self.GrabbableObject`) _asbp_grabbable_object)))))

(event `/Game/Player/I_InteractibleCharacter.Grab`
  (params (Value :type Boolean))
  (bind _grabbabletarget (`self.GrabbableTarget`))
  ;[0.2131 0.9103 1] Actions
  ;;[1 1 1] Grab/Release Behavior
  (if Value
    (`/Engine/EditorBlueprintResources/StandardMacros.IsValid` _grabbabletarget
      (:`Is Valid`
        (`self.GrabObject` _grabbabletarget)
        (bind (_direction _alpha) (`Timeline|ReachTrunkTimeline` :!via `PlayFromStart` :!label _label_2)
          (:`Update`
            (`self.UpdateGrabbedObjectDuringTransition` _alpha))
          (:`Finished`
            (set `self.GrabbingTransition` false)))))
    (else
      (set `self.GrabbingTransition` false :!label _label_3)
      (`/Engine/EditorBlueprintResources/StandardMacros.IsValid` (`self.GrabbedObject`)
        (:`Is Valid`
          (`self.ReleaseGrabbedObject`)
          (goto _label_2 :!via `Stop`))))))

(event `self.Interactible.OnComponentEndOverlap`
  (params (OverlappedComponent :type "PrimitiveComponent Object Reference") (OtherActor :type "Actor Object Reference") (OtherComp :type "PrimitiveComponent Object Reference") (OtherBodyIndex :type Integer))
  ;[1 0.1451 0.8144] Updates & Collisions
  ;;[1 1 1] When an object leave, we make sur to remove it from the list
  (if (`KismetSystemLibrary.DoesImplementInterface` OtherActor "/Game/Player/I_GameplayTagContainer.I_GameplayTagContainer_C")
    (bind _tags (message `/Game/Player/I_GameplayTagContainer.RetrieveTags` OtherActor))
    (if (`BlueprintGameplayTagLibrary.HasTag` _tags (struct :`TagName` "Elephantiquarry.Object.ObjectType.Grabable") true)
      (bind _asbp_grabbable_object (cast `/Game/Blueprints/Objects/BP_GrabbableObject` OtherActor))
      (`KismetArrayLibrary.Array_RemoveItem` (`self.GrabbableObject`) _asbp_grabbable_object))))

(event `OnGrabbedObjectDestroyed`
  ;[0.2131 0.9103 1] Actions
  ;;[1 1 1] Grab/Release Behavior
  (goto _label_3))

(event `self.CapsuleCollision.OnComponentHit`
  (params (HitComponent :type "PrimitiveComponent Object Reference") (OtherActor :type "Actor Object Reference") (OtherComp :type "PrimitiveComponent Object Reference") (NormalImpulse :type "Vector Structure") (Hit :type "HitResult Structure (by ref)"))
  ;[1 0.1451 0.8144] Updates & Collisions
)

(event `/Game/Player/I_InteractibleCharacter.Rotate`
  (params (Value :type "Vector2D Structure") (isController :type Boolean))
  ;[0.2131 0.9103 1] Actions
  ;;[1 1 1] Look Behavior
  (if (`self.isGrabbing`)
    (if (not (`self.GrabbingTransition`))
      (if isController
        (bind _returnvalue (`self.ProcessLookGamepadInput` Value))
        (bind (_dampenedlookx _dampenedlooky) (`self.DampenLookInput` (`KismetMathLibrary.BreakVector2D` _returnvalue) (`.Y` (`KismetMathLibrary.BreakVector2D` _returnvalue))))
        (set `self.LookInput` (`KismetMathLibrary.MakeVector2D` _dampenedlookx _dampenedlooky))
        (else
          (bind _returnvalue_2 (`self.ProcessLookKeyboardInput` Value))
          (bind (_dampenedlookx_2 _dampenedlooky_2) (`self.DampenLookInput` (`KismetMathLibrary.BreakVector2D` _returnvalue_2) (`.Y` (`KismetMathLibrary.BreakVector2D` _returnvalue_2))))
          (set `self.LookInput` (`KismetMathLibrary.MakeVector2D` _dampenedlookx_2 _dampenedlooky_2))))
      (`PrimitiveComponent.AddTorqueInDegrees` (`self.CapsuleCollision`) (`KismetMathLibrary.MakeVector` 0.0 0.0 (`self.ProcessLookToTorqueValue`)) "None" true))))

(fn `GetIdealGrabbableObject`
  (returns (Object :type "/Game/Blueprints/Objects/BP_GrabbableObject Object Reference"))
  (locals (closestToAlignment :type "Float (double-precision)" :default 999999.0) (closestToCenter :type "Float (double-precision)" :default 9999999.0) (currentSelectedActor :type "/Game/Blueprints/Objects/BP_GrabbableObject Object Reference") (MarginInDegrees :type Integer :default 10))
  (bind (_returnvalue_x _returnvalue_y) (`KismetMathLibrary.BreakVector` (`self.K2_GetActorLocation`)))
  (for _array_element (`self.GrabbableObject`)
    (bind _returnvalue (`self.IsGrabbableObjectAccessible` _array_element))
    (if _returnvalue
      (bind _returnvalue_2 (`self.GetSafeGrabbableObjectAngle` _array_element))
      (if (and (< (`self.GetAngleWithMargin` _returnvalue_2 (`local.MarginInDegrees`)) (`self.GetAngleWithMargin` (`local.closestToAlignment`) (`local.MarginInDegrees`))) (< _returnvalue_2 (/ (`self.InteractionConeAngle`) 2.0)))
        (set `local.closestToAlignment` _returnvalue_2 :!label _label)
        (bind (_returnvalue_x_2 _returnvalue_y_2) (`KismetMathLibrary.BreakVector` (`self.K2_GetActorLocation` _array_element)))
        (bind _returnvalue_3 (`KismetMathLibrary.Vector_DistanceSquared` (`KismetMathLibrary.MakeVector` _returnvalue_x_2 _returnvalue_y_2) (`KismetMathLibrary.MakeVector` _returnvalue_x _returnvalue_y)))
        (set `local.closestToCenter` _returnvalue_3)
        (set `local.currentSelectedActor` _array_element)
        (elif (and (<= (`self.GetAngleWithMargin` _returnvalue_2 (`local.MarginInDegrees`)) (`self.GetAngleWithMargin` (`local.closestToAlignment`) (`local.MarginInDegrees`))) (< _returnvalue_2 (/ (`self.InteractionConeAngle`) 2.0)))
          (if (< _returnvalue_3 (`local.closestToCenter`))
            (goto _label))))))
  (return (`local.currentSelectedActor`)))

(fn `GetSafeGrabbableObjectAngle`
  (params (GrabObject :type "/Game/Blueprints/Objects/BP_GrabbableObject Object Reference"))
  (returns (ReturnValue :type "Float (double-precision)"))
  (bind (_returnvalue_x _returnvalue_y) (`KismetMathLibrary.BreakVector` (`SceneComponent.K2_GetComponentLocation` (`self.CapsuleCollision`))))
  (bind _object (`/Game/Blueprints/Objects/BP_Object.GetPhysicsObject` GrabObject))
  (bind (_returnvalue_x_2 _returnvalue_y_2) (`KismetMathLibrary.BreakVector` (`SceneComponent.K2_GetComponentLocation` _object)))
  (bind _returnvalue (- (`KismetMathLibrary.MakeVector` _returnvalue_x_2 _returnvalue_y_2) (`KismetMathLibrary.MakeVector` _returnvalue_x _returnvalue_y)))
  (if (`KismetMathLibrary.NotEqualExactly_VectorVector` _returnvalue)
    (return (`KismetMathLibrary.DegAcos` (`KismetMathLibrary.Dot_VectorVector` (`SceneComponent.GetForwardVector` (`self.CapsuleCollision`)) (`KismetMathLibrary.Vector_NormalUnsafe` _returnvalue))))
    (else
      (return 10000.0))))

(fn `GrabObject`
  (params (GrabbableTarget :type "/Game/Blueprints/Objects/BP_GrabbableObject Object Reference"))
  (set `self.GrabbedObject` GrabbableTarget)
  (`/Game/Blueprints/Objects/BP_GrabbableObject.SetAsTarget` (`self.GrabbedObject`) false)
  (set `self.isGrabbing` true)
  (`/Game/Blueprints/Objects/BP_GrabbableObject.SetGrabbed` (`self.GrabbedObject`) true)
  (add `/Game/Blueprints/Objects/BP_Object.OnObjectDestroyed` (`self.GrabbedObject`) (`|CreateDelegate` :!event `OnGrabbedObjectDestroyed`))
  ;[1 1 1] Play Grab SFX
  (`FMODAudioComponent.Play` (`self.FMODAudio_Grab`))
  (`self.UpdateElephantStatsBasedOnGrabObject`)
  (set `self.GrabbingTransition` true)
  ;[1 1 1] Setting up collision type to Pawn means the player will ignore the objects mass when it collides with it, which avoids a lot of problems
  (bind _object (`/Game/Blueprints/Objects/BP_Object.GetPhysicsObject` (`self.GrabbedObject`)))
  (`PrimitiveComponent.SetCollisionObjectType` _object "ECC_Pawn")
  (`self.OnChangeGrab` true))

(fn `IsGrabbableObjectAccessible`
  (params (GrabbableObject :type "/Game/Blueprints/Objects/BP_Object Object Reference"))
  (returns (ReturnValue :type Boolean))
  (bind _capsulecollision (`self.CapsuleCollision`))
  (bind _returnvalue (+ (`SceneComponent.K2_GetComponentLocation` _capsulecollision) (`KismetMathLibrary.MakeVector` 0.0 0.0 (* (`CapsuleComponent.GetScaledCapsuleHalfHeight` _capsulecollision) 2.0))))
  ;[1 1 1] We linetrace in the direction of the object, but farther away and from a higher point
  (bind _object (`/Game/Blueprints/Objects/BP_Object.GetPhysicsObject` GrabbableObject))
  (bind _outpointonbody (`PrimitiveComponent.GetClosestPointOnCollision` _object _returnvalue "None"))
  ;[1 1 1] Sphere trace instead of line trace to get better results, and only the objects
  (bind _outhit (`KismetSystemLibrary.SphereTraceSingle` _returnvalue (+ _returnvalue (* (- _outpointonbody _returnvalue) (1.5 1.5 1.5))) 0.0 "TraceTypeQuery3"))
  (if (== (`.HitActor` (`GameplayStatics.BreakHitResult` _outhit)) GrabbableObject)
    ;[1 1 1] We then do a clean line trace on visibility to check if there's a wall
    (bind _outhit_2 (`KismetSystemLibrary.LineTraceSingle` _returnvalue (+ _outpointonbody (* (- (`.ImpactPoint` (`GameplayStatics.BreakHitResult` _outhit)) _returnvalue) (1.3 1.3 1.3))) "TraceTypeQuery1"))
    (return (== (`.HitActor` (`GameplayStatics.BreakHitResult` _outhit_2)) GrabbableObject))
    (else
      (return false))))

(fn `OnEventReleaseGrabbedObject`
  (params (ConstraintIndex :type Integer))
  (`self.ReleaseGrabbedObject`))

(fn `ProcessLookGamepadInput`
  (params (A :type "Vector2D Structure"))
  (returns (ReturnValue :type "Vector2D Structure"))
  (return (`KismetMathLibrary.GetRotated2D` A 90.0)))

(fn `ProcessLookKeyboardInput`
  (params (A :type "Vector2D Structure"))
  (returns (ReturnValue :type "Vector2D Structure"))
  (bind _returnvalue (`WidgetLayoutLibrary.GetMousePositionOnViewport`))
  (bind (_returnvalue_x _returnvalue_y) (`KismetMathLibrary.BreakVector2D` (- _returnvalue (`GameplayStatics.ProjectWorldToScreen` (`GameplayStatics.GetPlayerController` 0) (`SceneComponent.K2_GetComponentLocation` (`self.CapsuleCollision`))))))
  (return (`KismetMathLibrary.GetRotated2D` (`KismetMathLibrary.Normal2D` (`KismetMathLibrary.MakeVector2D` _returnvalue_x _returnvalue_y)) 90.0)))

(fn `ReleaseGrabbedObject`
  (`|ExecutionSequence`
    (:`then_0`
      ;[1 1 1] We reset our transition state and the physics object collision type to start behaving normally again
      (bind _object (`/Game/Blueprints/Objects/BP_Object.GetPhysicsObject` (`self.GrabbedObject`)))
      (`PrimitiveComponent.SetCollisionObjectType` _object "ECC_PhysicsBody"))
    (:`then_1`
      ;[1 1 1] We release the object from our handle (which makes it zero gravity and everything)
      (`PhysicsHandleComponent.ReleaseComponent` (`self.PhysicsHandle`)))
    (:`then_2`
      ;[1 1 1] Warn the object and ourselves we're not grabbing anymore
      (set `self.isGrabbing` false)
      (`/Game/Blueprints/Objects/BP_GrabbableObject.SetGrabbed` (`self.GrabbedObject`) false)
      (set `self.GrabbedObject` null)
      ;[1 1 1] Play Release SFX
      (`FMODAudioComponent.Play` (`self.FMODAudio_Release`)))
    (:`then_3`
      ;[1 1 1] When everything is done, we reset our rotation and speed parameters and notify everyone grabbing is finished
      (`self.ResetRotationAndSpeed`)
      (`self.OnChangeGrab` false))))

(fn `ResetRotationAndSpeed`
  (set `self.CurrentSpeedMultiplier` (`self.BaseSpeedMultiplier`))
  (set `self.CurrentRotationStrength` (`self.BaseRotationStrength`)))

(fn `UpdateElephantStatsBasedOnGrabObject`
  (bind (_returnvalue_x _returnvalue_y _returnvalue_z) (`KismetMathLibrary.BreakVector` (`SceneComponent.K2_GetComponentLocation` (`self.GrabbingPlace`))))
  (bind _object (`/Game/Blueprints/Objects/BP_Object.GetPhysicsObject` (`self.GrabbedObject`)))
  (bind _returnvalue (`PrimitiveComponent.GetMass` _object))
  (`TimelineComponent.SetPlayRate` (`self.ReachTrunkTimeline`) (`KismetMathLibrary.MapRangeClamped` _returnvalue 10.0 400.0 5.0 1.0))
  (set `self.CurrentRotationStrength` (`KismetMathLibrary.MapRangeClamped` _returnvalue 10.0 400.0 (`self.BaseRotationStrength`) 0.2))
  (set `self.CurrentSpeedMultiplier` (`KismetMathLibrary.MapRangeClamped` _returnvalue 10.0 400.0 (`self.BaseSpeedMultiplier`) 0.5))
  (bind _output_get (set `self.GrabbedItemHeight` (`KismetMathLibrary.MapRangeClamped` _returnvalue 100.0 400.0 0.0 (* (`CapsuleComponent.CapsuleHalfHeight` (`self.CapsuleCollision`)) -1.3))))
  (set `self.GrabPlacement` (`PrimitiveComponent.GetClosestPointOnCollision` _object (`SceneComponent.K2_GetComponentLocation` (`self.CapsuleCollision`)) "None"))
  (set `self.RagdollTargetLoc` (`KismetMathLibrary.InverseTransformLocation` (`SceneComponent.K2_GetComponentToWorld` (`self.CapsuleCollision`)) (`KismetMathLibrary.MakeVector` _returnvalue_x _returnvalue_y (+ _returnvalue_z _output_get))))
  (`PhysicsHandleComponent.GrabComponentAtLocation` (`self.PhysicsHandle`) _object "None" (`self.GrabPlacement`))
  (return))

(fn `UpdateGrabbedObjectDuringTransition`
  (params (Alpha :type "Float (single-precision)"))
  (bind _capsulecollision (`self.CapsuleCollision`))
  (`PhysicsHandleComponent.SetTargetLocation` (`self.PhysicsHandle`) (`KismetMathLibrary.VLerp` (`self.GrabPlacement`) (`KismetMathLibrary.TransformLocation` (`SceneComponent.K2_GetComponentToWorld` (`self.CapsuleCollision`)) (`self.RagdollTargetLoc`)) Alpha))
  (`SceneComponent.K2_SetWorldRotation` _capsulecollision (`KismetMathLibrary.RLerp` (`SceneComponent.K2_GetComponentRotation` _capsulecollision) (`KismetMathLibrary.FindLookAtRotation` (`SceneComponent.K2_GetComponentLocation` (`self.CapsuleCollision`)) (`self.GrabPlacement`)) Alpha true) false false))

(fn `UserConstructionScript`)