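; Player controller for the elephant character that sets up Enhanced Input and handles the end of a level.
; Forwards move, grab and rotate (mouse or controller) input to the pawn through interface messages, avoiding casts and stored references.
; On level finish, it spawns BP_ElephantCapture, layers fade and result widgets into the HUD container, then adds the menu mapping context.
; Click-to-move and cursor/touch helper functions exist but are not called here.
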(event `self.ReceiveBeginPlay`
  (bind _returnvalue (subsystem `EnhancedInputLocalPlayerSubsystem`))
  ;[0.05098 0.05098 0.05098] Add Mapping Context
  (`WidgetBlueprintLibrary.SetInputMode_GameOnly` self)
  (`/Engine/EditorBlueprintResources/StandardMacros.IsValid` _returnvalue
    (:`Is Valid`
      (`EnhancedInputSubsystemInterface.AddMappingContext` _returnvalue "/Game/Input/Elephant/IMC_Default.IMC_Default" 0 (struct)))))

(event `EnhancedInput|/Game/Input/Elephant/Actions/IA_Move`
  (params (ActionValue :type "Vector2D Structure") (ElapsedSeconds :type "Float (double-precision)") (TriggeredSeconds :type "Float (double-precision)") (InputAction :type "InputAction Object Reference" :default "/Game/Input/Elephant/Actions/IA_Move.IA_Move"))
  ;[1 1 1] Using an interface for the calls, that way we don't store a variable for the character and we don't cast it each time we want to use it
  (:`Triggered`
    (message `/Game/Player/I_InteractibleCharacter.Move` (`self.K2_GetPawn`) ActionValue :!label _label))
  (:`Started`
    (goto _label))
  (:`Ongoing`
    (goto _label))
  (:`Canceled`
    (goto _label))
  (:`Completed`
    (goto _label)))

(event `EnhancedInput|/Game/Input/Elephant/Actions/IA_Grab`
  (params (ActionValue :type Boolean) (ElapsedSeconds :type "Float (double-precision)") (TriggeredSeconds :type "Float (double-precision)") (InputAction :type "InputAction Object Reference" :default "/Game/Input/Elephant/Actions/IA_Grab.IA_Grab"))
  (bind _returnvalue (`self.K2_GetPawn`))
  ;[1 1 1] Using an interface for the calls, that way we don't store a variable for the character and we don't cast it each time we want to use it
  (:`Started`
    (message `/Game/Player/I_InteractibleCharacter.Grab` _returnvalue true))
  (:`Completed`
    (`WidgetBlueprintLibrary.SetInputMode_GameOnly` self)
    (message `/Game/Player/I_InteractibleCharacter.Grab` _returnvalue false)))

(event `EnhancedInput|/Game/Input/Elephant/Actions/IA_Rotate`
  (params (ActionValue :type "Vector2D Structure") (ElapsedSeconds :type "Float (double-precision)") (TriggeredSeconds :type "Float (double-precision)") (InputAction :type "InputAction Object Reference" :default "/Game/Input/Elephant/Actions/IA_Rotate.IA_Rotate"))
  ;[1 1 1] Using an interface for the calls, that way we don't store a variable for the character and we don't cast it each time we want to use it
  (:`Triggered`
    (message `/Game/Player/I_InteractibleCharacter.Rotate` (`self.K2_GetPawn`) ActionValue true :!label _label_2))
  (:`Started`
    (message `/Game/Player/I_InteractibleCharacter.StartedRotating` (`self.K2_GetPawn`)))
  (:`Ongoing`
    (goto _label_2))
  (:`Completed`
    (message `/Game/Player/I_InteractibleCharacter.FinishedRotating` (`self.K2_GetPawn`))))

(event `EnhancedInput|/Game/Input/Elephant/Actions/IA_RotateMouse`
  (params (ActionValue :type "Vector2D Structure") (ElapsedSeconds :type "Float (double-precision)") (TriggeredSeconds :type "Float (double-precision)") (InputAction :type "InputAction Object Reference" :default "/Game/Input/Elephant/Actions/IA_RotateMouse.IA_RotateMouse"))
  (:`Triggered`
    (message `/Game/Player/I_InteractibleCharacter.Rotate` (`self.K2_GetPawn`) ActionValue false :!label _label_3))
  (:`Started`
    (goto _label_3))
  (:`Ongoing`
    (goto _label_3))
  (:`Completed`
    (goto _label_3)))

(event `OnLevelFinished`
  (bind _returnvalue (subsystem `EnhancedInputLocalPlayerSubsystem`))
  (`|SpawnActorFromClass` "/Game/Player/Intro/BP_ElephantCapture.BP_ElephantCapture_C" (`KismetMathLibrary.MakeTransform` (0.0 0.0 5000.0)) "Undefined" "MultiplyWithRoot" self (`GameplayStatics.GetPlayerCharacter` 0))
  (bind _returnvalue_2 (`|CreateWidget` "/Game/UI/Widgets/Intro/WB_SimpleFadeInEndResult.WB_SimpleFadeInEndResult_C" null "/Game/UI/UI_Ressource/Textures/EndResult/T_BackgroundFade.T_BackgroundFade"))
  (bind _container (message `/Game/UI/Widgets/HUD/I_ElephantHUD.GetParentUIContainer` (`self.GetHUD`)))
  (bind _returnvalue_3 (`CanvasPanel.AddChildToCanvas` _container _returnvalue_2))
  (`CanvasPanelSlot.SetOffsets` _returnvalue_3 (make `Margin` 0.0))
  (`CanvasPanelSlot.SetAnchors` _returnvalue_3 (make `Anchors` (0.0 0.0) (1.0 1.0)))
  (`KismetSystemLibrary.Delay` 0.5)
  (bind _returnvalue_4 (`|CreateWidget` "/Game/UI/Widgets/EndMenu/WB_EndResultScreen.WB_EndResultScreen_C"))
  (bind _container_2 (message `/Game/UI/Widgets/HUD/I_ElephantHUD.GetParentUIContainer` (`self.GetHUD`)))
  (bind _returnvalue_5 (`CanvasPanel.AddChildToCanvas` _container_2 _returnvalue_4))
  (`CanvasPanelSlot.SetOffsets` _returnvalue_5 (make `Margin` 0.0))
  (`CanvasPanelSlot.SetAnchors` _returnvalue_5 (make `Anchors` (0.0 0.0) (1.0 1.0)))
  (`/Engine/EditorBlueprintResources/StandardMacros.IsValid` _returnvalue
    (:`Is Valid`
      (`EnhancedInputSubsystemInterface.AddMappingContext` _returnvalue "/Game/Input/MainMenu/IMC_MainMenu.IMC_MainMenu" 0 (struct)))))

(fn `Follow`
  (params (Location :type "Vector Structure"))
  (bind _returnvalue (`self.K2_GetPawn`))
  (`Pawn.AddMovementInput` _returnvalue (`KismetMathLibrary.GetDirectionUnitVector` (`self.K2_GetActorLocation` _returnvalue) Location) 1.0 false))

(fn `GetLocationUnderCursor`
  (returns (Hit :type Boolean) (Location :type "Vector Structure"))
  (bind (_bblockinghit _binitialoverlap _time _distance _location) (`GameplayStatics.BreakHitResult` (`self.GetHitResultUnderCursorByChannel` "TraceTypeQuery1")))
  (return _bblockinghit _location))

(fn `GetLocationUnderFinger`
  (returns (Hit :type Boolean) (Location :type "Vector Structure"))
  (bind (_bblockinghit _binitialoverlap _time _distance _location) (`GameplayStatics.BreakHitResult` (`self.GetHitResultUnderFingerByChannel` "Touch1" "TraceTypeQuery1" false)))
  (return _bblockinghit _location))

(fn `MoveTo`
  (params (Location :type "Vector Structure"))
  (`AIBlueprintHelperLibrary.SimpleMoveToLocation` self Location)
  (`NiagaraFunctionLibrary.SpawnSystemAtLocation` (`self.FXCursor`) Location))

(fn `UserConstructionScript`)