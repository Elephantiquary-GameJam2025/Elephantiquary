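; Physics-driven player elephant pawn that moves, turns and grabs objects with its trunk.
; Movement applies damped, camera-relative force and torque to the capsule under extra gravity.
; Tick highlights the best overlapping grabbable by view cone, traces and preference for Orderable tags.
; Grabbing reels the object in via PhysicsHandle and a timeline, scales reel, speed and turning by mass, then pulls and rotates the elephant toward it.
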(event `self.ReceiveBeginPlay`
  ;[1 0.1451 0.8144] Updates & Collisions
  (`|ExecutionSequence`
    (:`then_0`
      (`TimelineComponent.SetPlayRate` (`self.ReachTrunkTimeline`) 5.0)
      (`self.ResetRotationAndSpeed`)
      (for _array_element (`PrimitiveComponent.GetOverlappingActors` (`self.Interactible`) "/Game/Blueprints/Objects/BP_GrabbableObject.BP_GrabbableObject_C")
        (`self.TryAddGrabbableObject` _array_element)))
    (:`then_1`
      (`KismetSystemLibrary.Delay` 0.2)
      (`SceneComponent.SetHiddenInGame` (`self.Mesh`) false false))))

(event `/Game/Player/I_InteractibleCharacter.Move`
  (params (Value :type "Vector2D Structure"))
  (bind (_movex _movey) (`self.ProcessAndDampenMoveInput` Value))
  ;[0.2131 0.9103 1] Actions
  ;;[1 1 1] Move Behavior
  (if (`self.GrabbingTransition`)
    _
    (elif (> (`KismetMathLibrary.VSize2DSquared` Value) 0.0)
      (`/Engine/EditorBlueprintResources/StandardMacros.IsValid` (`self.GetController`)
        (:`Is Valid`
          (`|ExecutionSequence`
            (:`then_0`
              (set `self.LastInput` (`KismetMathLibrary.MakeVector2D` _movex _movey)))
            (:`then_1`
              (`PrimitiveComponent.AddForce` (`self.CapsuleCollision`) (`self.ScaleMoveInputToForce` _movex _movey) "None" false))
            (:`then_2`
              ;;;[1 1 1] If no input is pressed, we ignore the velocity based rotation
              (if (> (`KismetMathLibrary.VSize2DSquared` (`self.LastInput`)) 0.0)
                ;;;[1 1 1] Velocity based rotation of the character
                (if (and (`self.RotatesAutomatically`) (not (`self.isGrabbing`)))
                  (`PrimitiveComponent.AddTorqueInDegrees` (`self.CapsuleCollision`) (`KismetMathLibrary.MakeVector` 0.0 0.0 (`self.ProcessVelocityToTorqueValue`)) "None" true)))))))
      (else
        (set `self.LastInput` (0.0 0.0))))))

(event `self.ReceiveTick`
  (params (DeltaSeconds :type "Float (single-precision)"))
  ;[1 0.1451 0.8144] Updates & Collisions
  (`|ExecutionSequence`
    (:`then_0`
      (`PrimitiveComponent.AddForce` (`self.CapsuleCollision`) (0.0 0.0 -1000.0) "None" true) ; Artificially increasing gravity
    )
    (:`then_1`
      (if (`self.isGrabbing`)
        ;;[1 1 1] If we are grabbing, we stop looking for objects and instead update the location the grabbed object should be
        (if (not (`self.GrabbingTransition`))
          (`PhysicsHandleComponent.SetTargetLocation` (`self.PhysicsHandle`) (`SceneComponent.K2_GetComponentLocation` (`self.GrabbingPlace`)))
          (`self.UpdateTrunkPosition` (`SceneComponent.K2_GetComponentLocation` (`/Game/Blueprints/Objects/BP_GrabbableObject.TrunkPosTarget` (`self.GrabbedObject`))))
          (`self.AttractElephantTowardGrabbedObject`)
          (`self.RotateElephantTowardObject`))
        ;;[1 1 1] unless we are in grabbing transition (meaning we grabbed it but it didn't yet reach its grabbed position)
        (`/Engine/EditorBlueprintResources/StandardMacros.IsValid` (`self.GrabbableTarget`) :!label _label
          (:`Is Valid`
            (`/Game/Blueprints/Objects/BP_GrabbableObject.SetAsTarget` (`self.GrabbableTarget`) false)
            (set `self.GrabbableTarget` null)))
        (else
          ;;[1 1 1] If we're currently not grabbing, we are constantly searching for the object to highlight as grabbable
          (bind _object (`self.GetIdealGrabbableObject`))
          (`/Engine/EditorBlueprintResources/StandardMacros.IsValid` _object
            (:`Is Valid`
              (`/Engine/EditorBlueprintResources/StandardMacros.IsValid` (`self.GrabbableTarget`)
                (:`Is Valid`
                  (`/Game/Blueprints/Objects/BP_GrabbableObject.SetAsTarget` (`self.GrabbableTarget`) false))
                (:`Is Not Valid`
                  _))
              (bind _output_get (set `self.GrabbableTarget` _object))
              (`/Game/Blueprints/Objects/BP_GrabbableObject.SetAsTarget` _output_get true))
            (:`Is Not Valid`
              (goto _label))))))))

(event `/Game/Player/I_InteractibleCharacter.Grab`
  (params (Value :type Boolean))
  ;[0.2131 0.9103 1] Actions
  ;;[1 1 1] Grab/Release Behavior
  (if Value
    (`/Engine/EditorBlueprintResources/StandardMacros.IsValid` (`self.GrabbableTarget`)
      (:`Is Valid`
        (`self.GrabObject` (`self.GrabbableTarget`))
        (bind (_direction _alpha) (`Timeline|ReachTrunkTimeline` :!via `PlayFromStart` :!label _label_2)
          (:`Update`
            (`self.UpdateGrabbedObjectDuringTransition` _alpha)
            (`/Engine/EditorBlueprintResources/StandardMacros.IsValid` (`self.GrabbedObject`)
              (:`Is Valid`
                (`self.UpdateTrunkPosition` (`SceneComponent.K2_GetComponentLocation` (`/Game/Blueprints/Objects/BP_GrabbableObject.TrunkPosTarget` (`self.GrabbedObject`)))))
              (:`Is Not Valid`
                (`KismetSystemLibrary.PrintString` "ERROR : Grabbed object is null duiring transition" true true (struct :`R` 1.0 :`A` 1.0) 6.0))))
          (:`Finished`
            (set `self.GrabbingTransition` false)))))
    (else
      (set `self.GrabbingTransition` false :!label _label_3)
      (`/Engine/EditorBlueprintResources/StandardMacros.IsValid` (`self.GrabbedObject`)
        (:`Is Valid`
          (`self.ReleaseGrabbedObject`)
          (goto _label_2 :!via `Stop`))))))

(event `OnGrabbedObjectDestroyed`
  ;[0.2131 0.9103 1] Actions
  ;;[1 1 1] Grab/Release Behavior
  (goto _label_3))

(event `TryAddGrabbableObject`
  (params (Object :type "Actor Object Reference"))
  ;[1 0.1451 0.8144] Updates & Collisions
  (`self.AddGrabbableObjectToObjectsInRange` Object))

(event `/Game/Player/I_InteractibleCharacter.Rotate`
  (params (Value :type "Vector2D Structure") (isController :type Boolean))
  ;[0.2131 0.9103 1] Actions
  ;;[1 1 1] Look Behavior
  (if (`self.isGrabbing`)
    (if (not (`self.GrabbingTransition`))
      (if isController
        (bind _returnvalue (`self.ProcessLookGamepadInput` Value))
        (bind (_dampenedlookx _dampenedlooky) (`self.DampenLookInput` (`KismetMathLibrary.BreakVector2D` _returnvalue) (`.Y` (`KismetMathLibrary.BreakVector2D` _returnvalue))))
        (set `self.LookInput` (`KismetMathLibrary.MakeVector2D` _dampenedlookx _dampenedlooky))
        (else
          (bind _returnvalue_2 (`self.ProcessLookKeyboardInput` Value))
          (bind (_dampenedlookx_2 _dampenedlooky_2) (`self.DampenLookInput` (`KismetMathLibrary.BreakVector2D` _returnvalue_2) (`.Y` (`KismetMathLibrary.BreakVector2D` _returnvalue_2))))
          (set `self.LookInput` (`KismetMathLibrary.MakeVector2D` _dampenedlookx_2 _dampenedlooky_2))))
      (`PrimitiveComponent.AddTorqueInDegrees` (`self.CapsuleCollision`) (`KismetMathLibrary.MakeVector` 0.0 0.0 (`self.ProcessLookToTorqueValue` (`self.LookInput`) (`self.CurrentRotationStrength`))) "None" true))))

(event `self.Interactible.OnComponentBeginOverlap`
  (params (OverlappedComponent :type "PrimitiveComponent Object Reference") (OtherActor :type "Actor Object Reference") (OtherComp :type "PrimitiveComponent Object Reference") (OtherBodyIndex :type Integer) (bFromSweep :type Boolean) (SweepResult :type "HitResult Structure (by ref)"))
  ;[1 0.1451 0.8144] Updates & Collisions
  ;;[1 1 1] If an object enters our Interactible Capsule, this means it is a candidate to be grabbable, so we check if it has the right conditions and add it to the grabbable candidates
  (`self.AddGrabbableObjectToObjectsInRange` OtherActor))

(event `self.Interactible.OnComponentEndOverlap`
  (params (OverlappedComponent :type "PrimitiveComponent Object Reference") (OtherActor :type "Actor Object Reference") (OtherComp :type "PrimitiveComponent Object Reference") (OtherBodyIndex :type Integer))
  ;[1 0.1451 0.8144] Updates & Collisions
  ;;[1 1 1] When an object leave, we make sure to remove it from the list
  (if (`KismetSystemLibrary.DoesImplementInterface` OtherActor "/Game/Player/I_GameplayTagContainer.I_GameplayTagContainer_C")
    (bind _tags (message `/Game/Player/I_GameplayTagContainer.RetrieveTags` OtherActor))
    (if (`BlueprintGameplayTagLibrary.HasTag` _tags (struct :`TagName` "Elephantiquarry.Object.ObjectType.Grabable") true)
      (bind _asbp_grabbable_object (cast `/Game/Blueprints/Objects/BP_GrabbableObject` OtherActor))
      (`KismetArrayLibrary.Array_RemoveItem` (`self.GrabbableObjectsInRange`) _asbp_grabbable_object))))

(event `self.CapsuleCollision.OnComponentHit`
  (params (HitComponent :type "PrimitiveComponent Object Reference") (OtherActor :type "Actor Object Reference") (OtherComp :type "PrimitiveComponent Object Reference") (NormalImpulse :type "Vector Structure") (Hit :type "HitResult Structure (by ref)"))
  ;[1 0.1451 0.8144] Updates & Collisions
)

(fn `AddGrabbableObjectToObjectsInRange`
  (params (Object :type "Actor Object Reference"))
  (if (`KismetSystemLibrary.DoesImplementInterface` Object "/Game/Player/I_GameplayTagContainer.I_GameplayTagContainer_C")
    (bind _tags (message `/Game/Player/I_GameplayTagContainer.RetrieveTags` Object))
    (if (`BlueprintGameplayTagLibrary.HasTag` _tags (struct :`TagName` "Elephantiquarry.Object.ObjectType.Grabable") true)
      (bind _asbp_grabbable_object (cast `/Game/Blueprints/Objects/BP_GrabbableObject` Object))
      (if (`/Game/Blueprints/Objects/BP_GrabbableObject.IsGrabbable` _asbp_grabbable_object)
        (`KismetArrayLibrary.Array_Add` (`self.GrabbableObjectsInRange`) _asbp_grabbable_object)))))

(fn `AttractElephantTowardGrabbedObject`
  (bind (_returnvalue_x _returnvalue_y) (`KismetMathLibrary.BreakVector` (* (* (`self.GetAttractionStrengthByGrabbedObjectDistance`) (`self.GrabAttractionForce`)) (- (`self.K2_GetActorLocation` (`self.GrabbedObject`)) (`self.K2_GetActorLocation`)))))
  (`PrimitiveComponent.AddForce` (`self.CapsuleCollision`) (`KismetMathLibrary.MakeVector` _returnvalue_x _returnvalue_y) "None" false))

(fn `GetAttractionStrengthByGrabbedObjectDistance`
  (returns (ReturnValue :type "Float (single-precision)"))
  (bind (_returnvalue_x _returnvalue_y) (`KismetMathLibrary.BreakVector` (`self.K2_GetActorLocation`)))
  (bind (_returnvalue_x_2 _returnvalue_y_2) (`KismetMathLibrary.BreakVector` (`SceneComponent.K2_GetComponentLocation` (`/Game/Blueprints/Objects/BP_GrabbableObject.TrunkPosTarget` (`self.GrabbedObject`)))))
  (return (`CurveFloat.GetFloatValue` (`self.ElephantAttractionCurve`) (/ (`KismetMathLibrary.Vector_Distance` (`KismetMathLibrary.MakeVector` _returnvalue_x _returnvalue_y) (`KismetMathLibrary.MakeVector` _returnvalue_x_2 _returnvalue_y_2)) (`self.MaxGrabDistance`)))))

(fn `GetIdealGrabbableObject`
  (returns (Object :type "/Game/Blueprints/Objects/BP_GrabbableObject Object Reference"))
  (locals (ClosestToAlignment :type "Float (double-precision)" :default 999999.0) (ClosestToCenter :type "Float (double-precision)" :default 9999999.0) (IdealGrabbable :type "/Game/Blueprints/Objects/BP_GrabbableObject Object Reference") (IdealIsOrderable :type Boolean :default false) (MarginInDegrees :type Integer :default 10) (CandidateGrabbable :type "/Game/Blueprints/Objects/BP_GrabbableObject Object Reference") (CandidateIsOrderable :type Boolean :default false))
  (for _array_element (`self.GrabbableObjectsInRange`)
    (set `local.CandidateGrabbable` _array_element)
    ;[1 1 1] If candidate is not reachable we ignore it
    (bind _returnvalue (`self.IsGrabbableObjectAccessible` (`local.CandidateGrabbable`))) ; Checking for object in front or wall
    (if _returnvalue
      (bind _returnvalue_2 (`self.GetSafeGrabbableObjectAngle` (`local.CandidateGrabbable`)))
      ;[1 1 1] If candidate is not in interaction angle we ignore it
      (if (`self.IsAngleInInteractionRange` _returnvalue_2)
        (set `local.CandidateIsOrderable` (`BlueprintGameplayTagLibrary.HasTag` (`/Game/Blueprints/Objects/BP_Object.GameplayTagContainer` (`local.CandidateGrabbable`)) (struct :`TagName` "Elephantiquarry.Object.ObjectType.Orderable")))
        ;[1 1 1] Check if candidate is closer angle-wise
        (if (< (`self.GetAngleWithMargin` _returnvalue_2 (`local.MarginInDegrees`)) (`self.GetAngleWithMargin` (`local.ClosestToAlignment`) (`local.MarginInDegrees`)))
          ;[1 1 1] Setting a new best candidate - Ideal can be a non orderable object only if previous wasn't a non orderable as well
          (if (`local.CandidateIsOrderable`)
            (set `local.ClosestToAlignment` _returnvalue_2 :!label _label)
            (set `local.ClosestToCenter` (`self.GetObjectToElephantDistance` (`local.CandidateGrabbable`)))
            (set `local.IdealGrabbable` (`local.CandidateGrabbable`))
            (set `local.IdealIsOrderable` (`local.CandidateIsOrderable`))
            (else
              (if (not (`local.IdealIsOrderable`)) :!label _label_2
                (goto _label))))
          (elif (`local.CandidateIsOrderable`)
            (goto _label_2))))))
  (return (`local.IdealGrabbable`)))

(fn `GetObjectToElephantDistance`
  (params (Object :type "Actor Object Reference"))
  (returns (ReturnValue :type "Float (double-precision)"))
  (bind (_returnvalue_x _returnvalue_y) (`KismetMathLibrary.BreakVector` (`self.K2_GetActorLocation`)))
  (bind (_returnvalue_x_2 _returnvalue_y_2) (`KismetMathLibrary.BreakVector` (`self.K2_GetActorLocation` Object)))
  (return (`KismetMathLibrary.Vector_DistanceSquared` (`KismetMathLibrary.MakeVector` _returnvalue_x_2 _returnvalue_y_2) (`KismetMathLibrary.MakeVector` _returnvalue_x _returnvalue_y))))

(fn `GetSafeGrabbableObjectAngle`
  (params (GrabObject :type "/Game/Blueprints/Objects/BP_GrabbableObject Object Reference"))
  (returns (ReturnValue :type "Float (double-precision)"))
  (bind (_returnvalue_x _returnvalue_y) (`KismetMathLibrary.BreakVector` (`SceneComponent.K2_GetComponentLocation` (`self.CapsuleCollision`))))
  (bind _object (`/Game/Blueprints/Objects/BP_Object.GetPhysicsObject` GrabObject))
  (bind (_returnvalue_x_2 _returnvalue_y_2) (`KismetMathLibrary.BreakVector` (`SceneComponent.K2_GetComponentLocation` _object)))
  (bind _returnvalue (- (`KismetMathLibrary.MakeVector` _returnvalue_x_2 _returnvalue_y_2) (`KismetMathLibrary.MakeVector` _returnvalue_x _returnvalue_y)))
  (if (`KismetMathLibrary.NotEqualExactly_VectorVector` _returnvalue)
    (return (`KismetMathLibrary.DegAcos` (`KismetMathLibrary.Dot_VectorVector` (`SceneComponent.GetForwardVector` (`self.CapsuleCollision`)) (`KismetMathLibrary.Vector_NormalUnsafe` _returnvalue))))
    (else
      (return 10000.0))))

(fn `GrabObject`
  (params (GrabbableTarget :type "/Game/Blueprints/Objects/BP_GrabbableObject Object Reference"))
  (set `self.GrabbedObject` GrabbableTarget)
  (`/Game/Blueprints/Objects/BP_GrabbableObject.SetAsTarget` (`self.GrabbedObject`) false)
  (set `self.isGrabbing` true)
  (`/Game/Blueprints/Objects/BP_GrabbableObject.SetGrabbed` (`self.GrabbedObject`) true)
  (add `/Game/Blueprints/Objects/BP_Object.OnObjectDestroyed` (`self.GrabbedObject`) (`|CreateDelegate` :!event `OnGrabbedObjectDestroyed`))
  ;[1 1 1] Play Grab SFX
  (`FMODAudioComponent.Play` (`self.FMODAudio_Grab`))
  (`self.UpdateElephantStatsBasedOnGrabObject`)
  (set `self.GrabbingTransition` true)
  ;[1 1 1] Setting up collision type to Pawn means the player will ignore the objects mass when it collides with it, which avoids a lot of problems
  (bind _object (`/Game/Blueprints/Objects/BP_Object.GetPhysicsObject` (`self.GrabbedObject`)))
  (`PrimitiveComponent.SetCollisionObjectType` _object "ECC_Pawn")
  (`self.OnChangeGrab` true))

(fn `IsAngleInInteractionRange`
  (params (Angle :type "Float (double-precision)"))
  (returns (ReturnValue :type Boolean))
  (return (< Angle (/ (`self.InteractionConeAngle`) 2.0))))

(fn `IsGrabbableObjectAccessible`
  (params (GrabbableObject :type "/Game/Blueprints/Objects/BP_Object Object Reference"))
  (returns (ReturnValue :type Boolean))
  (bind _capsulecollision (`self.CapsuleCollision`))
  (bind _returnvalue (+ (`SceneComponent.K2_GetComponentLocation` _capsulecollision) (`KismetMathLibrary.MakeVector` 0.0 0.0 (* (`CapsuleComponent.GetScaledCapsuleHalfHeight` _capsulecollision) 2.0))))
  ;[1 1 1] We linetrace in the direction of the object, but farther away and from a higher point
  (bind _object (`/Game/Blueprints/Objects/BP_Object.GetPhysicsObject` GrabbableObject))
  (bind _outpointonbody (`PrimitiveComponent.GetClosestPointOnCollision` _object _returnvalue "None"))
  ;[1 1 1] Sphere trace instead of line trace to get better results, and only the objects
  (bind _outhit (`KismetSystemLibrary.SphereTraceSingle` _returnvalue (+ _returnvalue (* (- _outpointonbody _returnvalue) (1.5 1.5 1.5))) 0.0 "TraceTypeQuery3"))
  (if (== (`.HitActor` (`GameplayStatics.BreakHitResult` _outhit)) GrabbableObject)
    ;[1 1 1] We then do a clean line trace on visibility to check if there's a wall
    (bind _outhit_2 (`KismetSystemLibrary.LineTraceSingle` _returnvalue (+ _outpointonbody (* (- (`.ImpactPoint` (`GameplayStatics.BreakHitResult` _outhit)) _returnvalue) (1.3 1.3 1.3))) "TraceTypeQuery1"))
    (return (== (`.HitActor` (`GameplayStatics.BreakHitResult` _outhit_2)) GrabbableObject))
    (else
      (return false))))

(fn `OnEventReleaseGrabbedObject`
  (params (ConstraintIndex :type Integer))
  (`self.ReleaseGrabbedObject`))

(fn `ProcessLookGamepadInput`
  (params (A :type "Vector2D Structure"))
  (returns (ReturnValue :type "Vector2D Structure"))
  (return (`KismetMathLibrary.GetRotated2D` A 90.0)))

(fn `ProcessLookKeyboardInput`
  (params (A :type "Vector2D Structure"))
  (returns (ReturnValue :type "Vector2D Structure"))
  (bind _returnvalue (`WidgetLayoutLibrary.GetMousePositionOnViewport`))
  (bind (_returnvalue_x _returnvalue_y) (`KismetMathLibrary.BreakVector2D` (- _returnvalue (`GameplayStatics.ProjectWorldToScreen` (`GameplayStatics.GetPlayerController` 0) (`SceneComponent.K2_GetComponentLocation` (`self.CapsuleCollision`))))))
  (return (`KismetMathLibrary.GetRotated2D` (`KismetMathLibrary.Normal2D` (`KismetMathLibrary.MakeVector2D` _returnvalue_x _returnvalue_y)) 90.0)))

(fn `ReleaseGrabbedObject`
  (`|ExecutionSequence`
    (:`then_0`
      ;[1 1 1] We reset our transition state and the physics object collision type to start behaving normally again
      (bind _object (`/Game/Blueprints/Objects/BP_Object.GetPhysicsObject` (`self.GrabbedObject`)))
      (`PrimitiveComponent.SetCollisionObjectType` _object "ECC_PhysicsBody"))
    (:`then_1`
      ;[1 1 1] We release the object from our handle (which makes it zero gravity and everything)
      (`PhysicsHandleComponent.ReleaseComponent` (`self.PhysicsHandle`)))
    (:`then_2`
      ;[1 1 1] Warn the object and ourselves we're not grabbing anymore
      (set `self.isGrabbing` false)
      (`/Game/Blueprints/Objects/BP_GrabbableObject.SetGrabbed` (`self.GrabbedObject`) false)
      (set `self.GrabbedObject` null)
      ;[1 1 1] Play Release SFX
      (`FMODAudioComponent.Play` (`self.FMODAudio_Release`)))
    (:`then_3`
      ;[1 1 1] When everything is done, we reset our rotation and speed parameters and notify everyone grabbing is finished
      (`self.ResetRotationAndSpeed`)
      (`self.OnChangeGrab` false))))

(fn `ResetRotationAndSpeed`
  (set `self.CurrentSpeedMultiplier` (`self.BaseSpeedMultiplier`))
  (set `self.CurrentRotationStrength` (`self.BaseRotationStrength`)))

(fn `RotateElephantTowardObject`
  (bind (_returnvalue_x _returnvalue_y) (`KismetMathLibrary.BreakVector` (- (`self.K2_GetActorLocation` (`self.GrabbedObject`)) (`self.K2_GetActorLocation`))))
  (`PrimitiveComponent.AddTorqueInDegrees` (`self.CapsuleCollision`) (`KismetMathLibrary.MakeVector` 0.0 0.0 (* (`self.ProcessLookToTorqueValue` (`KismetMathLibrary.MakeVector2D` _returnvalue_x _returnvalue_y) (* (`self.CurrentRotationStrength`) 2.0)) (`KismetMathLibrary.Abs` (* (- (`KismetMathLibrary.Vector_CosineAngle2D` (- (`SceneComponent.K2_GetComponentLocation` (`/Game/Blueprints/Objects/BP_GrabbableObject.TrunkPosTarget` (`self.GrabbedObject`))) (`self.K2_GetActorLocation`)) (`SceneComponent.GetForwardVector` (`self.CapsuleCollision`))) 1.0) 0.5)))) "None" true))

(fn `StartTrunkExtensionSound`)

(fn `StopTrunkExtensionSound`)

(fn `TrunkExtensionSoundTick`)

(fn `UpdateElephantStatsBasedOnGrabObject`
  (locals (GrabbedObjectMesh :type "StaticMeshComponent Object Reference"))
  (bind _returnvalue (`PrimitiveComponent.GetMass` (`local.GrabbedObjectMesh`)))
  (bind _object (`/Game/Blueprints/Objects/BP_Object.GetPhysicsObject` (`self.GrabbedObject`)))
  (set `local.GrabbedObjectMesh` _object)
  (`TimelineComponent.SetPlayRate` (`self.ReachTrunkTimeline`) (`KismetMathLibrary.MapRangeClamped` _returnvalue 10.0 400.0 5.0 1.0))
  (set `self.CurrentRotationStrength` (`KismetMathLibrary.MapRangeClamped` _returnvalue 10.0 400.0 (`self.BaseRotationStrength`) 0.2))
  (set `self.CurrentSpeedMultiplier` (`KismetMathLibrary.MapRangeClamped` _returnvalue 10.0 400.0 (`self.BaseSpeedMultiplier`) 0.5))
  (`SceneComponent.K2_SetWorldLocation` (`/Game/Blueprints/Objects/BP_GrabbableObject.TrunkPosTarget` (`self.GrabbedObject`)) (`PrimitiveComponent.GetClosestPointOnCollision` (`local.GrabbedObjectMesh`) (`SceneComponent.K2_GetComponentLocation` (`self.CapsuleCollision`)) "None") false true)
  (`PhysicsHandleComponent.GrabComponentAtLocation` (`self.PhysicsHandle`) (`local.GrabbedObjectMesh`) "None" (`SceneComponent.K2_GetComponentLocation` (`/Game/Blueprints/Objects/BP_GrabbableObject.TrunkPosTarget` (`self.GrabbedObject`))))
  (return))

(fn `UpdateGrabbedObjectDuringTransition`
  (params (Alpha :type "Float (single-precision)"))
  (locals (AlphaLocal :type "Float (single-precision)"))
  (set `local.AlphaLocal` Alpha)
  (`PhysicsHandleComponent.SetTargetLocation` (`self.PhysicsHandle`) (`KismetMathLibrary.VLerp` (`SceneComponent.K2_GetComponentLocation` (`/Game/Blueprints/Objects/BP_GrabbableObject.TrunkPosTarget` (`self.GrabbedObject`))) (`SceneComponent.K2_GetComponentLocation` (`self.GrabbingPlace`)) (`local.AlphaLocal`)))
  (`SceneComponent.K2_SetWorldRotation` (`self.CapsuleCollision`) (`KismetMathLibrary.RLerp` (`SceneComponent.K2_GetComponentRotation` (`self.CapsuleCollision`)) (`KismetMathLibrary.FindLookAtRotation` (`SceneComponent.K2_GetComponentLocation` (`self.CapsuleCollision`)) (`SceneComponent.K2_GetComponentLocation` (`/Game/Blueprints/Objects/BP_GrabbableObject.TrunkPosTarget` (`self.GrabbedObject`)))) (`local.AlphaLocal`) true) false false))

(fn `UserConstructionScript`)