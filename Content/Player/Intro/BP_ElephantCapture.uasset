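; BP_ElephantCapture is an intro actor that shows an animated, rotating elephant mesh for a scene capture component.
; On BeginPlay it loops the Anim_Stompy_Fatigued animation and resizes the capture's render target to match the viewport size.
; Each tick it yaws the skeletal mesh by RotationRate scaled by delta time, producing a steady turntable spin.
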(event `self.ReceiveBeginPlay`
  (bind (_returnvalue_x _returnvalue_y) (`KismetMathLibrary.BreakVector2D` (`WidgetLayoutLibrary.GetViewportSize`)))
  (`SkeletalMeshComponent.PlayAnimation` (`self.SkeletalMesh`) "/Game/3Dassets/Anims/Anim_Stompy_Fatigued.Anim_Stompy_Fatigued" true)
  (`KismetRenderingLibrary.ResizeRenderTarget2D` (`SceneCaptureComponent2D.TextureTarget` (`self.SceneCaptureComponent2D`)) (`KismetMathLibrary.FTrunc` _returnvalue_x) (`KismetMathLibrary.FTrunc` _returnvalue_y)))

(event `self.ReceiveTick`
  (params (DeltaSeconds :type "Float (single-precision)"))
  (`SceneComponent.K2_AddRelativeRotation` (`self.SkeletalMesh`) (`KismetMathLibrary.MakeRotator` 0.0 0.0 (* (`self.RotationRate`) DeltaSeconds)) false false))

(fn `UserConstructionScript`)